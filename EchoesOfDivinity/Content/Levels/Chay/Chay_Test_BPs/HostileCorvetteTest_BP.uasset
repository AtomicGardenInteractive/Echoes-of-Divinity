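; Test enemy corvette AI pawn that chases a sensed TestShip_BP and fires missiles at it.
; PawnSensing triggers an AI move to within range, then spawns both a HostileMissile and a Missile_BP from MissilePort.
; A DoOnce gates the attack and resets five seconds after a successful move.
; The first damage event zeroes health regardless of amount and destroys the corvette, as damage subtraction is unwired.
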(event OnSeePawn(PawnSensing)
  (params (Pawn :type Pawn%20Object%20Reference))
  (bind _missileport (Variables|Default|GetMissilePort))
  (bind _returnvalue (Transformation|GetWorldTransform _missileport))
  (bind _astest_ship_bp (Utilities|Casting|CastToTestShip_BP Pawn))
  (Development|PrintString "Ship Sensed")
  (Utilities|FlowControl|DoOnce false :!label _label
    (:Completed
      (AI|AIMoveTo self "0, 0, 0" _astest_ship_bp 2e+03 false
        (:OnSuccess
          (Development|PrintString "Range Reached")
          (CallFunction|FireMissile)
          (Game|SpawnActorfromClass "/Game/Assets/3D/Blueprints/Missile_BP.Missile_BP_C" (Math|Transform|MakeTransform (.location _returnvalue) (.rotation _returnvalue) "1.000000,1.000000,1.000000") "AlwaysSpawn" self 0)
          (Utilities|FlowControl|Delay 5.0)
          (goto _label Reset))))))

(event EventBeginPlay)

(event Collision|EventActorBeginOverlap
  (params (OtherActor :type Actor%20Object%20Reference)))

(event EventTick
  (params (DeltaSeconds :type Float%20%28single-precision%29)))

(event MouseInput|EventActorOnClicked
  (params (ButtonPressed :type Key%20Structure :default "None")))

(event Game|Damage|EventAnyDamage
  (params (Damage :type Float%20%28single-precision%29) (DamageType :type Damage%20Type%20Object%20Reference) (InstigatedBy :type Controller%20Object%20Reference) (DamageCauser :type Actor%20Object%20Reference))
  (Utilities|FlowControl|DoOnce false
    (:Completed
      (if (not (Variables|Default|GetHostileIsDead))
        (bind _output_get (Variables|Default|SetCurrenthealth (Math|Float|Clamp(Float) 0.0 0.0 (Variables|Default|GetMaxHealth))))
        (Development|PrintString (Utilities|String|ToString(Float) _output_get))
        (if (== _output_get 0.0)
          (Utilities|Casting|CastToPlayerController_BP (Game|GetPlayerController 0))
          (Variables|Default|SetHostileIsDead true)
          (Actor|DestroyActor))))))

(fn ConstructionScript
  (if (not (Variables|Default|GetIsPlayerUnit))
    _))

(fn FireMissile
  (bind _missileport (Variables|Default|GetMissilePort))
  (bind _returnvalue (Transformation|GetWorldTransform _missileport))
  (Game|SpawnActorfromClass "/Game/Levels/Chay/Chay_Test_BPs/HostileMissile.HostileMissile_C" (Math|Transform|MakeTransform (.location _returnvalue) (.rotation _returnvalue) "1.000000,1.000000,1.000000") "AlwaysSpawn" self 0))