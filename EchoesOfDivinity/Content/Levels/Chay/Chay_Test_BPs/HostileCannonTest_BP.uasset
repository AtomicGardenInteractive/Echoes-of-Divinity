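; Test hostile cannon turret that automatically tracks and fires on player-side BP_Ship_P actors within sensing range.
; Each Tick a sphere overlap and line-of-sight check picks the last visible ship found, as the distance comparison never filters for nearest.
; The turret rotates toward it at constant speed.
; A DoOnce with delays paces shots, spawning a bullet, railgun Niagara effect and sound at the Arrow.
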(event EventBeginPlay)

(event Collision|EventActorBeginOverlap
  (params (OtherActor :type Actor%20Object%20Reference)))

(event EventTick
  (params (DeltaSeconds :type Float%20%28single-precision%29))
  (bind _arrow (Variables|Default|GetArrow))
  (bind _returnvalue (Transformation|GetWorldTransform _arrow))
  (CallFunction|FindBestTargetHostile)
  (Variables|Default|GetOurTarget
    (:then
      (CallFunction|UpdateHostileTurretRotation DeltaSeconds)
      (Utilities|FlowControl|DoOnce false :!label _label
        (:Completed
          (Utilities|FlowControl|Delay 5.0)
          (Game|SpawnActorfromClass "/Game/Assets/3D/Blueprints/Projectiles/BP_Bullet_P.BP_Bullet_P_C" (Math|Transform|MakeTransform (.location _returnvalue) (.rotation _returnvalue) "1.000000,1.000000,1.000000") "AlwaysSpawn" self 0)
          (Niagara|SpawnSystematLocation "/Game/Assets/3D/VFX/Niagara/NS_RailgunFire.NS_RailgunFire" (.location _returnvalue) (.rotation _returnvalue))
          (Audio|PlaySoundatLocation "/Game/Assets/Audio/WAVs/RailgunFire2_mixdown.RailgunFire2_mixdown" (.location _returnvalue) "0, 0, 0" 1.0 1.0 0.0 0 0 0 0)
          (Utilities|FlowControl|Delay 2.0)
          (goto _label Reset))))
    (:else)))

(fn ConstructionScript)

(fn UpdateHostileTurretRotation
  (params (DeltaSeconds :type Float%20%28double-precision%29))
  (Transformation|SetWorldRotation (Variables|Default|GetTurret) (Class|KismetMathLibrary|RInterptoConstant (Transformation|GetWorldRotation (Variables|Default|GetTurret)) (Math|Rotator|FindLookatRotation (Transformation|GetWorldLocation (Variables|Default|GetTurret)) (Transformation|GetActorLocation (Variables|Default|GetOurTarget))) DeltaSeconds (Variables|Default|GetRotationSpeed)) false false))

(fn FindBestTargetHostile
  (LocalVariables|SetBestDistance%28Local%29 (+ (Variables|Default|GetSensingRange) 1.0))
  (bind _outactors (Collision|SphereOverlapActors (Transformation|GetActorLocation) (Variables|Default|GetSensingRange) (Utilities|Array|MakeArray "ObjectTypeQuery8") "/Game/Assets/3D/Blueprints/Ships/BP_Ship_P.BP_Ship_P_C")) ; Actors to ignore can be used to...ignore...acotrs, if you want to do that
  (for _array_element _outactors
    (bind _output_get (LocalVariables|SetCurrentTarget%28Local%29 _array_element))
    (LocalVariables|SetCurrentDistance%28Local%29 (Transformation|GetDistanceTo _output_get self))
    (if (or (< 0.0 (LocalVariables|GetBestDistance%28Local%29)) (not (Utilities|IsValid (LocalVariables|GetBestTarget%28Local%29))))
      (bind _result (CallFunction|HasLineOfSight (Transformation|GetWorldLocation (Variables|Default|GetTurret)) (Transformation|GetActorLocation (LocalVariables|GetCurrentTarget%28Local%29)) (Utilities|Array|MakeArray self (LocalVariables|GetCurrentTarget%28Local%29))))
      (if _result
        (LocalVariables|SetBestTarget%28Local%29 (LocalVariables|GetCurrentTarget%28Local%29))
        (LocalVariables|SetBestDistance%28Local%29 (LocalVariables|GetCurrentDistance%28Local%29)))))
  (Variables|Default|SetOurTarget (LocalVariables|GetBestTarget%28Local%29)))