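; BP_Probe is a projectile probe that deploys a light area and reveals hidden actors around it.
; Ten seconds after BeginPlay it stops its movement, rotates its mesh and spawns the NS_ProbeLightArea effect at the mesh.
; Every tick, from spawn onward, a zero-length sphere trace on a custom channel unhides the single actor it hits.
; The no-hit branch tries to re-hide that same trace's hit actor, so revealed actors effectively stay visible.
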(event EventBeginPlay
  (bind _staticmesh (Variables|Default|GetStaticMesh))
  (bind _returnvalue (Transformation|GetWorldTransform _staticmesh))
  (Utilities|FlowControl|Delay 1e+01)
  (Components|Movement|StopMovementImmediately (Variables|Default|GetProjectileMovement))
  (Transformation|SetRelativeRotation (Variables|Default|GetStaticMesh) "0.000000,90.000000,0.000000" false false)
  (Niagara|SpawnSystematLocation "/Game/Assets/3D/VFX/Niagara/NS_ProbeLightArea.NS_ProbeLightArea" (.location _returnvalue) (.rotation _returnvalue)))

(event Collision|EventActorBeginOverlap
  (params (OtherActor :type Actor%20Object%20Reference)))

(event EventTick
  (params (DeltaSeconds :type Float%20%28single-precision%29))
  (bind _returnvalue (Transformation|GetActorLocation))
  (bind (_outhit _returnvalue_2) (Collision|SphereTraceByChannel _returnvalue _returnvalue 7e+02 "TraceTypeQuery3" false 0 "None"))
  (if _returnvalue_2
    (Utilities|IsValid (.HitActor (Collision|BreakHitResult _outhit))
      (:Is%20Valid
        (Rendering|SetActorHiddenInGame (.HitActor (Collision|BreakHitResult _outhit)) false)))
    (else
      (Utilities|IsValid (.HitActor (Collision|BreakHitResult _outhit))
        (:Is%20Valid
          (Rendering|SetActorHiddenInGame (.HitActor (Collision|BreakHitResult _outhit)) true))))))

(fn ConstructionScript)