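; BP_Bullet_P is a projectile configured by a BulletTypes reference supplying mesh, lifespan-based range, initial speed, damage and type.
; Construction applies those settings and copies the owner's first tag, so overlaps with same-tagged actors are ignored.
; Other overlaps apply damage, then after a tiny delay spawn railgun impact effects and sound.
; A switch on bullet type then destroys small and large railgun slugs.
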(event Collision|EventActorBeginOverlap
  (params (OtherActor :type Actor%20Object%20Reference))
  (bind _staticmesh (Variables|Default|GetStaticMesh))
  (bind _returnvalue (Transformation|GetWorldTransform _staticmesh))
  (Utilities|IsValid OtherActor
    (:Is%20Valid
      (if (not (== (Utilities|Array|Get(acopy) (Variables|Actor|GetTags)) (Utilities|Array|Get(acopy) (Variables|/Script/Engine.Actor|GetTags OtherActor))))
        (Game|Damage|ApplyDamage OtherActor (Variables|/Game/Assets/3D/Blueprints/Data_Assets/Bullets/P_DataAsset_Bullets.P_DataAsset_Bullets_C|GetProjectile%20Damage (Variables|Default|GetBullet%20Types)) 0 self)
        (Utilities|FlowControl|Delay 0.01)
        (Niagara|SpawnSystematLocation "/Game/Assets/3D/VFX/Niagara/NS_RailgunImpact.NS_RailgunImpact" (.location _returnvalue) (.rotation _returnvalue) "0.050000,0.050000,0.050000")
        (Audio|SpawnSoundatLocation "/Game/Assets/Audio/WAVs/RailgunImpact3_mixdown.RailgunImpact3_mixdown" (.location (Transformation|GetWorldTransform (Variables|Default|GetStaticMesh))) "0, 0, 0" 1.0 1.0 0.0 0 0)
        (switch Utilities|FlowControl|Switch|SwitchonEN_Bullet_Types (Variables|/Game/Assets/3D/Blueprints/Data_Assets/Bullets/P_DataAsset_Bullets.P_DataAsset_Bullets_C|GetBullet%20Type (Variables|Default|GetBullet%20Types))
          (:NewEnumerator0
            _)
          (:NewEnumerator1
            _))
        (Actor|DestroyActor)))))

(fn ConstructionScript
  (bind _bullet_types (Variables|Default|GetBullet%20Types)
    (:then
      (Utilities|FlowControl|Sequence
        (:then_0
          (Components|StaticMesh|SetStaticMesh (Variables|Default|GetStaticMesh) (Variables|/Game/Assets/3D/Blueprints/Data_Assets/Bullets/P_DataAsset_Bullets.P_DataAsset_Bullets_C|GetBullet%20Mesh _bullet_types)))
        (:then_1
          (Actor|SetLifeSpan (Variables|/Game/Assets/3D/Blueprints/Data_Assets/Bullets/P_DataAsset_Bullets.P_DataAsset_Bullets_C|GetProjectile%20Range%20%28Life%20Span%29 _bullet_types)))
        (:then_2
          (Variables|/Script/Engine.ProjectileMovementComponent|SetInitialSpeed (Variables|Default|GetProjectileMovement) (Variables|/Game/Assets/3D/Blueprints/Data_Assets/Bullets/P_DataAsset_Bullets.P_DataAsset_Bullets_C|GetProjectile%20Speed _bullet_types)))
        (:then_3
          (Variables|Default|SetTags (Utilities|Array|MakeArray (Utilities|Array|Get(acopy) (Variables|/Script/Engine.Actor|GetTags (Components|GetOwner))))))))
    (:else)))