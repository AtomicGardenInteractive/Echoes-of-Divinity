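; Homing missile fired by a BP_Ship_P, configured from MissileType data for mesh, top speed, lifespan and damage.
; It enables homing on the ship's attack target after a short delay, then polls until that target is invalid and retargets once via a nearest-actor sphere search.
; The owner's first tag acts as team ID, filtering search and nose-collision damage.
; Each hit taken removes one health; impact or zero health destroys it with effects.
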(event OnComponentBeginOverlap(NoseCollision)
  (params (OverlappedComponent :type Primitive%20Component%20Object%20Reference) (OtherActor :type Actor%20Object%20Reference) (OtherComp :type Primitive%20Component%20Object%20Reference) (OtherBodyIndex :type Integer) (bFromSweep :type Boolean) (SweepResult :type Hit%20Result%20Structure%20%28by%20ref%29))
  (bind _self self)
  (bind _rootcomponent (Variables|Transformation|GetRootComponent _self))
  (bind _returnvalue (Transformation|GetWorldTransform _rootcomponent))
  ;[1 1 1] Missile Damage system
  (if (!= (Utilities|Array|Get(acopy) (Variables|/Script/Engine.Actor|GetTags OtherActor)) (Utilities|Array|Get(acopy) (Variables|Actor|GetTags)))
    (Game|Damage|ApplyDamage OtherActor (Variables|/Game/Assets/3D/Blueprints/Data_Assets/Missiles/P_DataAsset_Missiles.P_DataAsset_Missiles_C|GetProjectile%20Point%20Damage (Variables|Default|GetMissile%20Type)) 0 (Components|GetOwner))
    (Niagara|SpawnSystematLocation "/Game/Assets/3D/VFX/Niagara/BigExplosions/Niagara/NS_Air_1.NS_Air_1" (.location _returnvalue) (.rotation _returnvalue) "0.100000,0.100000,0.100000")
    (Actor|DestroyActor)))

(event Custom|Find%20New%20Lock%20On%20Target
  ;[1 1 1] Finds a new target in range
  (bind _homing_traget (CallFunction|FindNewHomingTarget))
  (Variables|/Script/Engine.ProjectileMovementComponent|SetHomingTargetComponent (Variables|Default|GetProjectileMovement) _homing_traget))

(event Game|Damage|EventAnyDamage
  (params (Damage :type Float%20%28single-precision%29) (DamageType :type Damage%20Type%20Object%20Reference) (InstigatedBy :type Controller%20Object%20Reference) (DamageCauser :type Actor%20Object%20Reference))
  (bind _missilecollision (Variables|Default|GetMissileCollision))
  (bind _returnvalue (Transformation|GetWorldLocation _missilecollision))
  ;[1 1 1] Missile Health
  (bind _output_get (Variables|Default|SetCurrentHealth (Math|Float|Clamp(Float) (- (Variables|Default|GetCurrentHealth) 1.0) 0.0 (Variables|Default|GetMaxHealth))))
  (if (<= _output_get 0.0)
    (Variables|Default|SetMissileIsDead true)
    (Niagara|SpawnSystematLocation "/Game/Assets/3D/VFX/Niagara/BigExplosions/Niagara/NS_Air_2.NS_Air_2" _returnvalue "0, 0, 0" "0.050000,0.050000,0.050000")
    (Audio|PlaySoundatLocation "/Game/Assets/Audio/WAVs/SingularExplosion_Missile__mixdown.SingularExplosion_Missile__mixdown" _returnvalue "0, 0, 0" 1.0 1.0 0.0 0 0 0 0)
    (Actor|DestroyActor)))

(event EventBeginPlay
  (bind _projectilemovement (Variables|Default|GetProjectileMovement))
  ;[1 1 1] Homming System
  (bind _asbp_ship_p (Utilities|Casting|CastToBP_Ship_P (Components|GetOwner)))
  (bind _attack_target (Variables|/Game/Assets/3D/Blueprints/Ships/BP_Ship_P.BP_Ship_P_C|GetAttack%20Target _asbp_ship_p)
    (:then
      (Variables|Default|SetTarget%20Actor _attack_target)
      (Variables|/Script/Engine.ProjectileMovementComponent|SetHomingTargetComponent _projectilemovement (Actor|GetComponentbyClass _attack_target "/Script/Engine.SceneComponent"))
      (Utilities|FlowControl|Delay 0.5)
      (Variables|/Script/Engine.ProjectileMovementComponent|SetbIsHomingProjectile _projectilemovement true)
      (Utilities|FlowControl|Delay 0.5 :!label _label)
      (Variables|Default|GetTarget%20Actor
        (:then
          (goto _label))
        (:else
          (CallFunction|FindNewLockonTarget))))
    (:else)))

(fn ConstructionScript
  (bind _missile_type (Variables|Default|GetMissile%20Type)
    (:then
      (Utilities|FlowControl|Sequence
        (:then_0
          (Components|StaticMesh|SetStaticMesh (Variables|Default|GetStaticMesh) (Variables|/Game/Assets/3D/Blueprints/Data_Assets/Missiles/P_DataAsset_Missiles.P_DataAsset_Missiles_C|GetMissile%20Mesh _missile_type)))
        (:then_1
          (Variables|Default|SetTags (Utilities|Array|MakeArray (Utilities|Array|Get(acopy) (Variables|/Script/Engine.Actor|GetTags (Components|GetOwner))))))
        (:then_2
          (Variables|/Script/Engine.ProjectileMovementComponent|SetMaxSpeed (Variables|Default|GetProjectileMovement) (Variables|/Game/Assets/3D/Blueprints/Data_Assets/Missiles/P_DataAsset_Missiles.P_DataAsset_Missiles_C|GetProjectile%20Max%20Speed _missile_type)))
        (:then_3
          (Actor|SetLifeSpan (Variables|/Game/Assets/3D/Blueprints/Data_Assets/Missiles/P_DataAsset_Missiles.P_DataAsset_Missiles_C|GetProjectile%20Range%20%28Life%20Span%29 _missile_type)))))
    (:else)))

(fn FindNewHomingTarget
  (bind _outactors (Actor|GetAllActorswithTag (Utilities|Array|Get(acopy) (Variables|/Script/Engine.Actor|GetTags (Components|GetOwner)))))
  (bind _outactors_2 (Collision|SphereOverlapActors (Transformation|GetActorLocation) 2e+03 (Utilities|Array|MakeArray "ObjectTypeQuery8") "/Script/Engine.Actor" _outactors))
  (for _array_element _outactors_2
    (if (< (Math|Vector|VectorLength (- (Transformation|GetActorLocation _array_element) (Transformation|GetActorLocation))) (Variables|Default|GetClosest%20Distance))
      (Variables|Default|SetClosest%20Distance (Math|Vector|VectorLength (- (Transformation|GetActorLocation _array_element) (Transformation|GetActorLocation))))
      (Variables|Default|SetTarget%20Actor _array_element)))
  (bind _target_actor (Variables|Default|GetTarget%20Actor)
    (:then
      (return (Actor|GetComponentbyClass _target_actor "/Script/Engine.SceneComponent")))
    (:else)))