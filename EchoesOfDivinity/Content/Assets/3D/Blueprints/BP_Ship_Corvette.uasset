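; Corvette ship Blueprint that handles the ship's weapon and probe launch events through the ACWeapons component.
; Missile events fire ShipData types from TorpedoLauncher, with types crossed: swarm fires CruiseMissileType and cruise fires SwarmMissileType.
; Probe launch spawns BP_Probe at ProbeLaunch, gated by a DoOnce that resets after a delay.
; Rail cannon and torpedo events are empty; their firing calls and the corvette widget logic are disconnected.
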(event EventBeginPlay
  (|CallParentFunction) ; This node is disabled and will not be called.\nDrag off pins to build functionality.
)

(event Collision|EventActorBeginOverlap
  (params (OtherActor :type Actor%20Object%20Reference)))

(event EventTick
  (params (DeltaSeconds :type Float%20%28single-precision%29)))

(event EventLaunchProbe
  ;[1 1 1] Weapons
  (Utilities|FlowControl|DoOnce false :!label _label
    (:Completed
      (for _array_element (Utilities|Array|MakeArray (Variables|Default|GetProbeLaunch))
        (Default|LaunchProbe (Variables|Default|GetAC_Weapons) "/Game/Assets/3D/Blueprints/BP_Probe.BP_Probe_C" _array_element)
        (Utilities|FlowControl|Delay 6e+01)
        (goto _label Reset)))))

(event EventLaunchSwarmMissile
  ;[1 1 1] Weapons
  (Default|FireMissile (Variables|Default|GetAC_Weapons) (Variables|/Game/Assets/3D/Blueprints/Data_Assets/Ships/P_DataAsset_Ships.P_DataAsset_Ships_C|GetCruise%20Missile%20Type (Variables|Default|GetShip%20Data)) (Variables|Default|GetTorpedoLauncher)))

(event EventLaunchCruiseMissile
  ;[1 1 1] Weapons
  (Default|FireMissile (Variables|Default|GetAC_Weapons) (Variables|/Game/Assets/3D/Blueprints/Data_Assets/Ships/P_DataAsset_Ships.P_DataAsset_Ships_C|GetSwarm%20Missile%20Type (Variables|Default|GetShip%20Data)) (Variables|Default|GetTorpedoLauncher)))

(event EventFireRailCannon
  ;[1 1 1] Weapons
)

(event EventLaunchTorpedo
  ;[1 1 1] Weapons
)

(fn ConstructionScript
  (|CallParentFunction))