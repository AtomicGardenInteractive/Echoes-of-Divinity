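; Actor component that tracks a ship's health as a hull total plus separate bow, bridge and stern pools.
; Each damage function subtracts from its pool and clamps to a caller-supplied maximum, with HullDamage returning true when the total hits zero.
; A depleted section calls CriticalDamage with zero damage, whose 0–1 clamp cuts total health to at most 1.
; No executed logic here initializes the pools.
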(event EventBeginPlay)

(event EventTick
  (params (DeltaSeconds :type Float%20%28single-precision%29)))

(fn HullDamage
  (params (Damage :type Float%20%28double-precision%29) (Total%20Health%20Max :type Float%20%28double-precision%29))
  (bind _output_get (Variables|Default|SetTotal%20Health%20Current (Math|Float|Clamp(Float) (- (Variables|Default|GetTotal%20Health%20Current) Damage) 0.0 Total%20Health%20Max)))
  (if (== _output_get 0.0)
    (return true)))

(fn BowDamage
  (params (Damage :type Float%20%28double-precision%29) (Bow%20Health%20Max :type Float%20%28double-precision%29))
  (bind _output_get (Variables|Default|SetBow%20Health%20Current (Math|Float|Clamp(Float) (- (Variables|Default|GetBow%20Health%20Current) Damage) 0.0 Bow%20Health%20Max)))
  (if (== _output_get 0.0)
    (CallFunction|CriticalDamage 0.0)))

(fn BridgeDamage
  (params (Damage :type Float%20%28double-precision%29) (Bridge%20Health%20Max :type Float%20%28double-precision%29))
  (bind _output_get (Variables|Default|SetBridge%20Health%20Current (Math|Float|Clamp(Float) (- (Variables|Default|GetBridge%20Health%20Current) Damage) 0.0 Bridge%20Health%20Max)))
  (if (== _output_get 0.0)
    (CallFunction|CriticalDamage 0.0)))

(fn SternDamage
  (params (Damage :type Float%20%28double-precision%29) (Stern%20Health%20Max :type Float%20%28double-precision%29))
  (bind _output_get (Variables|Default|SetStern%20Health%20Current (Math|Float|Clamp(Float) (- (Variables|Default|GetStern%20Health%20Current) Damage) 0.0 Stern%20Health%20Max)))
  (if (== _output_get 0.0)
    (CallFunction|CriticalDamage 0.0)))

(fn CriticalDamage
  (params (Damage :type Float%20%28double-precision%29))
  (Variables|Default|SetTotal%20Health%20Current (Math|Float|Clamp(Float) (- (Variables|Default|GetTotal%20Health%20Current) Damage))))