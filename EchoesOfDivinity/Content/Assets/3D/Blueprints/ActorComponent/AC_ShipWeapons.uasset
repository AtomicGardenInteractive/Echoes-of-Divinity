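; AC_ShipWeapons is an actor component that spawns cannon projectiles, missiles and probes for a ship.
; Each function spawns at a passed-in component's world location and rotation, ignoring collisions.
; Cannon class and scale come from WeaponData, while missiles use a passed class at fixed scale and print their name.
; LaunchProbe always spawns BP_Probe, ignoring its class input, and unlike the others sets no owner.
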(event EventBeginPlay)

(event EventTick
  (params (DeltaSeconds :type Float%20%28single-precision%29)))

(fn FireCannon
  (params (Weapon%20Data :type P%20Data%20Asset%20Weapons%20Object%20Reference) (Firing%20Point :type Scene%20Component%20Object%20Reference))
  (bind _returnvalue (Transformation|GetWorldTransform Firing%20Point))
  (Game|SpawnActorfromClass (Variables|/Game/Assets/3D/Blueprints/Data_Assets/Weapons/P_DataAsset_Weapons.P_DataAsset_Weapons_C|GetProjectile Weapon%20Data) (Math|Transform|MakeTransform (.location _returnvalue) (.rotation _returnvalue) (Variables|/Game/Assets/3D/Blueprints/Data_Assets/Weapons/P_DataAsset_Weapons.P_DataAsset_Weapons_C|GetProjectile%20Size Weapon%20Data)) "AlwaysSpawn" (Components|GetOwner) 0))

(fn FireMissile
  (params (Missile%20BP :type BP%20Missile%20P%20Fixed%20Class%20Reference) (Firing%20Point :type Scene%20Component%20Object%20Reference))
  (bind _returnvalue (Transformation|GetWorldTransform Firing%20Point))
  (bind _returnvalue_2 (Game|SpawnActorfromClass Missile%20BP (Math|Transform|MakeTransform (.location _returnvalue) (.rotation _returnvalue) "0.500000,0.500000,0.500000") "AlwaysSpawn" (Components|GetOwner) 0))
  (Development|PrintString (Utilities|GetDisplayName _returnvalue_2)))

(fn LaunchProbe
  (params (BP_Probe :type BP%20Probe%20Class%20Reference) (NewParam :type Scene%20Component%20Object%20Reference))
  (bind _returnvalue (Transformation|GetWorldTransform NewParam))
  (Game|SpawnActorfromClass "/Game/Assets/3D/Blueprints/BP_Probe.BP_Probe_C" (Math|Transform|MakeTransform (.location _returnvalue) (.rotation _returnvalue) "1.000000,1.000000,1.000000") "AlwaysSpawn" 0 0))