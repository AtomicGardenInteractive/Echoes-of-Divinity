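; Actor component that tracks a ship's health as a total hull pool plus bow, bridge and stern sections, initialized from ship type maximums.
; Damage functions clamp each pool, and every hit leaving a section at zero adds critical damage.
; At zero hull, HullDamage reports death and takes its exploded flag from Death.
; Death is an empty stub, with its ship removal and critical-damage-weighted random explosion roll left disconnected.
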(fn SetUpHealth
  (params (Ship%20Types :type P%20Data%20Asset%20Ships%20Object%20Reference))
  (Variables|Default|SetShip%20Types Ship%20Types)
  (Variables|Default|SetTotal%20Health%20Current (Variables|/Game/Assets/3D/Blueprints/Data_Assets/Ships/P_DataAsset_Ships.P_DataAsset_Ships_C|GetTotal%20Health%20Max (Variables|Default|GetShip%20Types)))
  (Variables|Default|SetBow%20Health%20Current (Variables|/Game/Assets/3D/Blueprints/Data_Assets/Ships/P_DataAsset_Ships.P_DataAsset_Ships_C|GetBow%20Health%20Max (Variables|Default|GetShip%20Types)))
  (Variables|Default|SetBridge%20Health%20Current (Variables|/Game/Assets/3D/Blueprints/Data_Assets/Ships/P_DataAsset_Ships.P_DataAsset_Ships_C|GetBridge%20Health%20Max (Variables|Default|GetShip%20Types)))
  (Variables|Default|SetStern%20Health%20Current (Variables|/Game/Assets/3D/Blueprints/Data_Assets/Ships/P_DataAsset_Ships.P_DataAsset_Ships_C|GetStern%20Health%20Max (Variables|Default|GetShip%20Types))))

(fn HullDamage
  (params (Damage :type Float%20%28double-precision%29))
  (bind _output_get (Variables|Default|SetTotal%20Health%20Current (Math|Float|Clamp(Float) (- (Variables|Default|GetTotal%20Health%20Current) Damage) 0.0 (Variables|/Game/Assets/3D/Blueprints/Data_Assets/Ships/P_DataAsset_Ships.P_DataAsset_Ships_C|GetTotal%20Health%20Max (Variables|Default|GetShip%20Types)))))
  (if (== _output_get 0.0)
    (bind _is_exploded (CallFunction|Death))
    (return (== _output_get 0.0) _is_exploded)))

(fn BowDamage
  (params (Damage :type Float%20%28double-precision%29))
  (bind _output_get (Variables|Default|SetBow%20Health%20Current (Math|Float|Clamp(Float) (- (Variables|Default|GetBow%20Health%20Current) Damage) 0.0 (Variables|/Game/Assets/3D/Blueprints/Data_Assets/Ships/P_DataAsset_Ships.P_DataAsset_Ships_C|GetBow%20Health%20Max (Variables|Default|GetShip%20Types)))))
  (if (== _output_get 0.0)
    (CallFunction|CriticalDamage 1.0)))

(fn BridgeDamage
  (params (Damage :type Float%20%28double-precision%29))
  (bind _output_get (Variables|Default|SetBridge%20Health%20Current (Math|Float|Clamp(Float) (- (Variables|Default|GetBridge%20Health%20Current) Damage) 0.0 (Variables|/Game/Assets/3D/Blueprints/Data_Assets/Ships/P_DataAsset_Ships.P_DataAsset_Ships_C|GetBridge%20Health%20Max (Variables|Default|GetShip%20Types)))))
  (if (== _output_get 0.0)
    (CallFunction|CriticalDamage 1.0)))

(fn SternDamage
  (params (Damage :type Float%20%28double-precision%29))
  (bind _output_get (Variables|Default|SetStern%20Health%20Current (Math|Float|Clamp(Float) (- (Variables|Default|GetStern%20Health%20Current) Damage) 0.0 (Variables|/Game/Assets/3D/Blueprints/Data_Assets/Ships/P_DataAsset_Ships.P_DataAsset_Ships_C|GetStern%20Health%20Max (Variables|Default|GetShip%20Types)))))
  (if (== _output_get 0.0)
    (CallFunction|CriticalDamage 1.0)))

(fn CriticalDamage
  (params (Damage :type Float%20%28double-precision%29))
  (Variables|Default|SetCritical%20Damage%20Current (+ Damage (Variables|Default|GetCritical%20Damage%20Current))))

(fn Death)