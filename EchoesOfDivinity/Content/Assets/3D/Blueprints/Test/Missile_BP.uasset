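; Homing missile that chases another TestShip_BP and deals damage to it on contact.
; A looping half-second delay from BeginPlay reruns the target search and feeds the result to ProjectileMovement as its homing target.
; The search scans all TestShip_BP actors, excluding the owning ship, for the closest one.
; Capsule overlap applies damage and destroys the missile only when the overlapped actor is the current target.
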(event OnComponentBeginOverlap(Capsule)
  (params (OverlappedComponent :type Primitive%20Component%20Object%20Reference) (OtherActor :type Actor%20Object%20Reference) (OtherComp :type Primitive%20Component%20Object%20Reference) (OtherBodyIndex :type Integer) (bFromSweep :type Boolean) (SweepResult :type Hit%20Result%20Structure%20%28by%20ref%29))
  (if (== OtherActor (Variables|Default|GetTarget%20Actor))
    (Game|Damage|ApplyDamage OtherActor 5e+01 0 (Components|GetOwner))
    (Actor|DestroyActor)))

(event Custom|Lock%20On%20Target
  (bind _projectilemovement (Variables|Default|GetProjectileMovement))
  (bind _homing_traget (CallFunction|FindHomingTarget))
  (Variables|/Script/Engine.ProjectileMovementComponent|SetHomingTargetComponent _projectilemovement _homing_traget)
  (Variables|/Script/Engine.ProjectileMovementComponent|SetbIsHomingProjectile _projectilemovement true))

(event EventBeginPlay
  (Utilities|FlowControl|Delay 0.5 :!label _label)
  (CallFunction|LockonTarget)
  (goto _label))

(fn ConstructionScript)

(fn FindHomingTarget
  (bind _outactors (Actor|GetAllActorsOfClass "/Game/Assets/3D/Blueprints/Test/TestShip_BP.TestShip_BP_C"))
  (bind _astest_ship_bp (Utilities|Casting|CastToTestShip_BP (Components|GetOwner)))
  (Utilities|Array|RemoveItem _outactors _astest_ship_bp)
  (for _array_element _outactors
    (if (< (Math|Vector|VectorLength (- (Transformation|GetActorLocation _array_element) (Transformation|GetActorLocation))) (Variables|Default|GetClosest%20Distance))
      (Variables|Default|SetClosest%20Distance (Math|Vector|VectorLength (- (Transformation|GetActorLocation _array_element) (Transformation|GetActorLocation))))
      (Variables|Default|SetTarget%20Actor _array_element)))
  (return (Actor|GetComponentbyClass (Variables|Default|GetTarget%20Actor) "/Script/Engine.SceneComponent")))