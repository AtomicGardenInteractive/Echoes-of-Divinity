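; Enemy destroyer ship Blueprint that adds cursor feedback and demo intro and win screens on top of its parent class.
; Hovering over the capsule switches the player's cursor to crosshairs.
; BeginPlay turns on the selection indicator and shows the Open Level widget for three minutes.
; The SelectionIndicatorOff event is repurposed as the win trigger, playing the end-demo audio and showing the win screen.
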(event OnBeginCursorOver(CapsuleComponent)
  (params (TouchedComponent :type Primitive%20Component%20Object%20Reference))
  ;[1 1 1] Change Cursor on mouse over
  (Variables|/Script/Engine.PlayerController|SetCurrentMouseCursor (Game|GetPlayerController 0) "Crosshairs"))

(event OnEndCursorOver(CapsuleComponent)
  (params (TouchedComponent :type Primitive%20Component%20Object%20Reference))
  ;[1 1 1] Change Cursor on mouse over
  (Variables|/Script/Engine.PlayerController|SetCurrentMouseCursor (Game|GetPlayerController 0) "Default"))

(event EventBeginPlay
  (|CallParentFunction)
  (CallFunction|SelectionIndicatoron)
  (Variables|/Script/Engine.PlayerController|SetbEnableMouseOverEvents (Game|GetPlayerController 0) true)
  ;[1 1 1] Display Open Level widget
  (bind _returnvalue (UserInterface|CreateWidget "/Game/Assets/UI/OnboardingLevel/WP_OpenLevel.WP_OpenLevel_C"))
  (UserInterface|Viewport|AddtoViewport _returnvalue 0)
  (Utilities|FlowControl|Delay 1.8e+02)
  (Widget|RemovefromParent _returnvalue))

(event Collision|EventActorBeginOverlap
  (params (OtherActor :type Actor%20Object%20Reference))
  (|CallParentFunction OtherActor) ; This node is disabled and will not be called.\nDrag off pins to build functionality.
)

(event EventTick
  (params (DeltaSeconds :type Float%20%28single-precision%29))
  (|CallParentFunction DeltaSeconds) ; This node is disabled and will not be called.\nDrag off pins to build functionality.
)

(event EventDestroyed)

(event EventSelectionIndicatorOff
  ;[1 1 1] Win Screen
  (Audio|PlaySound2D "/Game/Assets/Audio/WAVs/VoiceLines/ShipAI/AIEndDemo_mixdown.AIEndDemo_mixdown" 1.0 1.0 0.0 0 0)
  (bind _returnvalue (UserInterface|CreateWidget "/Game/Assets/UI/WP_DemoWinScreen.WP_DemoWinScreen_C"))
  (UserInterface|Viewport|AddtoViewport _returnvalue 0))

(fn ConstructionScript
  (|CallParentFunction))