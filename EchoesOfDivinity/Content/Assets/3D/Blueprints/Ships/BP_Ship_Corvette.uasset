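; Corvette ship Blueprint that adds torpedo and probe launch events on top of its parent class.
; Both events delegate to the ACWeapons component, with torpedoes taking type and size from ShipData and firing from the TorpedoLauncher point.
; Probes launch as BP_Probe from the ProbeLaunch point, gated by a DoOnce that resets after a one-minute delay to act as a cooldown.
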(event EventBeginPlay
  (|CallParentFunction))

(event Collision|EventActorBeginOverlap
  (params (OtherActor :type Actor%20Object%20Reference)))

(event EventTick
  (params (DeltaSeconds :type Float%20%28single-precision%29)))

(event EventLaunchProbe
  ;[1 1 1] Weapons
  (Utilities|FlowControl|DoOnce false :!label _label
    (:Completed
      (for _array_element (Utilities|Array|MakeArray (Variables|Default|GetProbeLaunch))
        (Default|LaunchProbe (Variables|Default|GetAC_Weapons) "/Game/Assets/3D/Blueprints/Projectiles/BP_Probe.BP_Probe_C" _array_element)
        (Utilities|FlowControl|Delay 6e+01)
        (goto _label Reset)))))

(event EventLaunchTorpedo
  (bind _ship_data (Variables|Default|GetShip%20Data))
  ;[1 1 1] Weapons
  (Default|FireMissile (Variables|Default|GetAC_Weapons) (Variables|/Game/Assets/3D/Blueprints/Data_Assets/Ships/P_DataAsset_Ships.P_DataAsset_Ships_C|GetTorpedo%20Type _ship_data) (Variables|Default|GetTorpedoLauncher) (Variables|/Game/Assets/3D/Blueprints/Data_Assets/Ships/P_DataAsset_Ships.P_DataAsset_Ships_C|GetTorpedo%20Size _ship_data)))

(fn ConstructionScript
  (|CallParentFunction))