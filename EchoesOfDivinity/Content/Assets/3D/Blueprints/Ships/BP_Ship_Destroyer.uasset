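; Destroyer ship Blueprint that adds a weapons HUD on BeginPlay and a defeat screen when destroyed.
; Fire events pass ShipData weapon types and launch points to ACWeapons for twin rail cannons, twin torpedoes and swarm missiles, plus a probe launcher.
; DoOnce gates with delayed resets provide cooldowns for all but torpedoes.
; Swarm missiles fire as staggered volleys from two launchers in parallel through a Sequence.
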(event EventBeginPlay
  (|CallParentFunction)
  (bind _returnvalue (UserInterface|CreateWidget "/Game/Assets/UI/ShipUI/WP_SimpleShipWeapons.WP_SimpleShipWeapons_C" 0 0))
  (UserInterface|Viewport|AddtoViewport _returnvalue 0))

(event Collision|EventActorBeginOverlap
  (params (OtherActor :type Actor%20Object%20Reference)))

(event EventFireRailCannon
  ;[1 1 1] Weapons
  (Utilities|FlowControl|DoOnce false :!label _label
    (:Completed
      (Utilities|FlowControl|Delay (Variables|/Game/Assets/3D/Blueprints/Data_Assets/Weapons/P_DataAsset_Weapons.P_DataAsset_Weapons_C|GetInital%20Firing%20Delay (Variables|/Game/Assets/3D/Blueprints/Data_Assets/Ships/P_DataAsset_Ships.P_DataAsset_Ships_C|GetRail%20Cannon%20Projectile%20Type (Variables|Default|GetShip%20Data))))
      (for _array_element (Utilities|Array|MakeArray (Variables|Default|GetRail%20Cannon%20Launch%20Pos%20Left) (Variables|Default|GetRail%20Cannon%20Launch%20Pos%20Right))
        (Default|FireCannon (Variables|Default|GetAC_Weapons) (Variables|/Game/Assets/3D/Blueprints/Data_Assets/Ships/P_DataAsset_Ships.P_DataAsset_Ships_C|GetRail%20Cannon%20Projectile%20Type (Variables|Default|GetShip%20Data)) _array_element))
      (Utilities|FlowControl|Delay (Variables|/Game/Assets/3D/Blueprints/Data_Assets/Weapons/P_DataAsset_Weapons.P_DataAsset_Weapons_C|GetDelay%20Between%20Rounds (Variables|/Game/Assets/3D/Blueprints/Data_Assets/Ships/P_DataAsset_Ships.P_DataAsset_Ships_C|GetRail%20Cannon%20Projectile%20Type (Variables|Default|GetShip%20Data))))
      (goto _label Reset))))

(event EventLaunchProbe
  ;[1 1 1] Weapons
  (Utilities|FlowControl|DoOnce false :!label _label
    (:Completed
      (for _array_element (Utilities|Array|MakeArray (Variables|Default|GetRail%20Cannon%20Launch%20Pos%20Right))
        (Default|LaunchProbe (Variables|Default|GetAC_Weapons) "/Game/Assets/3D/Blueprints/Projectiles/BP_Probe.BP_Probe_C" _array_element)
        (Utilities|FlowControl|Delay 6e+01)
        (goto _label Reset)))))

(event EventDestroyed
  (bind _returnvalue (UserInterface|CreateWidget "/Game/Assets/UI/WP_DefeatedScreen.WP_DefeatedScreen_C"))
  (UserInterface|Viewport|AddtoViewport _returnvalue 0))

(event EventLaunchTorpedo
  (bind _ship_data (Variables|Default|GetShip%20Data))
  ;[1 1 1] Weapons
  (for _array_element (Utilities|Array|MakeArray (Variables|Default|GetTorpedoLauncher) (Variables|Default|GetTorpedoLauncher1))
    (Default|FireMissile (Variables|Default|GetAC_Weapons) (Variables|/Game/Assets/3D/Blueprints/Data_Assets/Ships/P_DataAsset_Ships.P_DataAsset_Ships_C|GetTorpedo%20Type _ship_data) _array_element (Variables|/Game/Assets/3D/Blueprints/Data_Assets/Ships/P_DataAsset_Ships.P_DataAsset_Ships_C|GetTorpedo%20Size _ship_data))))

(event EventLaunchSwarmMissile
  (bind _returnvalue (+ 0.3 0.0))
  (bind _missilelauncher (Variables|Default|GetMissileLauncher))
  (bind _missilelauncher1 (Variables|Default|GetMissileLauncher1))
  (bind _ship_data (Variables|Default|GetShip%20Data))
  (bind _ship_data_2 (Variables|Default|GetShip%20Data))
  (bind _ship_data_3 (Variables|Default|GetShip%20Data))
  (bind _ship_data_4 (Variables|Default|GetShip%20Data))
  (bind _ship_data_5 (Variables|Default|GetShip%20Data))
  (bind _ship_data_6 (Variables|Default|GetShip%20Data))
  (bind _ship_data_7 (Variables|Default|GetShip%20Data))
  (bind _ship_data_8 (Variables|Default|GetShip%20Data))
  (bind _ship_data_9 (Variables|Default|GetShip%20Data))
  (bind _ship_data_10 (Variables|Default|GetShip%20Data))
  ;[1 1 1] Swarm Missiles
  (Utilities|FlowControl|DoOnce false :!label _label
    (:Completed
      (Audio|PlaySoundatLocation "/Game/Assets/Audio/WAVs/MissileSwarmLaunch3_mixdown.MissileSwarmLaunch3_mixdown" (Transformation|GetWorldLocation (Variables|Character|GetMesh)) "0, 0, 0" 1.0 1.0 0.0 0 0 0 0)
      (Utilities|FlowControl|Sequence
        (:then_0
          (Default|FireMissile (Variables|Default|GetAC_Weapons) (Variables|/Game/Assets/3D/Blueprints/Data_Assets/Ships/P_DataAsset_Ships.P_DataAsset_Ships_C|GetSwarm%20Missile%20Type _ship_data_6) _missilelauncher (Variables|/Game/Assets/3D/Blueprints/Data_Assets/Ships/P_DataAsset_Ships.P_DataAsset_Ships_C|GetSwarm%20Missile%20Size _ship_data_6))
          (Utilities|FlowControl|Delay _returnvalue)
          (Default|FireMissile (Variables|Default|GetAC_Weapons) (Variables|/Game/Assets/3D/Blueprints/Data_Assets/Ships/P_DataAsset_Ships.P_DataAsset_Ships_C|GetSwarm%20Missile%20Type _ship_data_8) _missilelauncher (Variables|/Game/Assets/3D/Blueprints/Data_Assets/Ships/P_DataAsset_Ships.P_DataAsset_Ships_C|GetSwarm%20Missile%20Size _ship_data_8))
          (Utilities|FlowControl|Delay _returnvalue)
          (Default|FireMissile (Variables|Default|GetAC_Weapons) (Variables|/Game/Assets/3D/Blueprints/Data_Assets/Ships/P_DataAsset_Ships.P_DataAsset_Ships_C|GetSwarm%20Missile%20Type _ship_data_7) _missilelauncher (Variables|/Game/Assets/3D/Blueprints/Data_Assets/Ships/P_DataAsset_Ships.P_DataAsset_Ships_C|GetSwarm%20Missile%20Size _ship_data_7))
          (Utilities|FlowControl|Delay _returnvalue)
          (Default|FireMissile (Variables|Default|GetAC_Weapons) (Variables|/Game/Assets/3D/Blueprints/Data_Assets/Ships/P_DataAsset_Ships.P_DataAsset_Ships_C|GetSwarm%20Missile%20Type _ship_data_9) _missilelauncher (Variables|/Game/Assets/3D/Blueprints/Data_Assets/Ships/P_DataAsset_Ships.P_DataAsset_Ships_C|GetSwarm%20Missile%20Size _ship_data_9))
          (Utilities|FlowControl|Delay _returnvalue)
          (Default|FireMissile (Variables|Default|GetAC_Weapons) (Variables|/Game/Assets/3D/Blueprints/Data_Assets/Ships/P_DataAsset_Ships.P_DataAsset_Ships_C|GetSwarm%20Missile%20Type _ship_data_10) _missilelauncher (Variables|/Game/Assets/3D/Blueprints/Data_Assets/Ships/P_DataAsset_Ships.P_DataAsset_Ships_C|GetSwarm%20Missile%20Size _ship_data_10)))
        (:then_1
          (Default|FireMissile (Variables|Default|GetAC_Weapons) (Variables|/Game/Assets/3D/Blueprints/Data_Assets/Ships/P_DataAsset_Ships.P_DataAsset_Ships_C|GetSwarm%20Missile%20Type _ship_data) _missilelauncher1 (Variables|/Game/Assets/3D/Blueprints/Data_Assets/Ships/P_DataAsset_Ships.P_DataAsset_Ships_C|GetSwarm%20Missile%20Size _ship_data))
          (Utilities|FlowControl|Delay _returnvalue)
          (Default|FireMissile (Variables|Default|GetAC_Weapons) (Variables|/Game/Assets/3D/Blueprints/Data_Assets/Ships/P_DataAsset_Ships.P_DataAsset_Ships_C|GetSwarm%20Missile%20Type _ship_data_4) _missilelauncher1 (Variables|/Game/Assets/3D/Blueprints/Data_Assets/Ships/P_DataAsset_Ships.P_DataAsset_Ships_C|GetSwarm%20Missile%20Size _ship_data_4))
          (Utilities|FlowControl|Delay _returnvalue)
          (Default|FireMissile (Variables|Default|GetAC_Weapons) (Variables|/Game/Assets/3D/Blueprints/Data_Assets/Ships/P_DataAsset_Ships.P_DataAsset_Ships_C|GetSwarm%20Missile%20Type _ship_data_3) _missilelauncher1 (Variables|/Game/Assets/3D/Blueprints/Data_Assets/Ships/P_DataAsset_Ships.P_DataAsset_Ships_C|GetSwarm%20Missile%20Size _ship_data_3))
          (Utilities|FlowControl|Delay _returnvalue)
          (Default|FireMissile (Variables|Default|GetAC_Weapons) (Variables|/Game/Assets/3D/Blueprints/Data_Assets/Ships/P_DataAsset_Ships.P_DataAsset_Ships_C|GetSwarm%20Missile%20Type _ship_data_5) _missilelauncher1 (Variables|/Game/Assets/3D/Blueprints/Data_Assets/Ships/P_DataAsset_Ships.P_DataAsset_Ships_C|GetSwarm%20Missile%20Size _ship_data_5))
          (Utilities|FlowControl|Delay _returnvalue)
          (Default|FireMissile (Variables|Default|GetAC_Weapons) (Variables|/Game/Assets/3D/Blueprints/Data_Assets/Ships/P_DataAsset_Ships.P_DataAsset_Ships_C|GetSwarm%20Missile%20Type _ship_data_2) _missilelauncher1 (Variables|/Game/Assets/3D/Blueprints/Data_Assets/Ships/P_DataAsset_Ships.P_DataAsset_Ships_C|GetSwarm%20Missile%20Size _ship_data_2))
          (Utilities|FlowControl|Delay 15.0)
          (goto _label Reset))))))

(fn ConstructionScript
  (|CallParentFunction))