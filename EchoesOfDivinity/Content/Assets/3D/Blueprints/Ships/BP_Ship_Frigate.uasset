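; Frigate ship Blueprint that exposes fire events for a rail cannon, torpedo, probe and swarm missile salvo.
; Each event passes a firing point to the ACWeapons component, with weapon types and sizes from ShipData except the fixed probe class.
; DoOnce gates reset after delays act as cooldowns, data-driven for the cannon and hardcoded for the others.
; The swarm fires five staggered missiles per trigger, and probes launch from the rail cannon point.
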(event EventBeginPlay
  (|CallParentFunction) ; This node is disabled and will not be called.\nDrag off pins to build functionality.
)

(event Collision|EventActorBeginOverlap
  (params (OtherActor :type Actor%20Object%20Reference)))

(event EventTick
  (params (DeltaSeconds :type Float%20%28single-precision%29)))

(event EventLaunchProbe
  ;[1 1 1] Weapons
  (Utilities|FlowControl|DoOnce false :!label _label
    (:Completed
      (for _array_element (Utilities|Array|MakeArray (Variables|Default|GetRail%20Cannon))
        (Default|LaunchProbe (Variables|Default|GetAC_Weapons) "/Game/Assets/3D/Blueprints/Projectiles/BP_Probe.BP_Probe_C" _array_element)
        (Utilities|FlowControl|Delay 6e+01)
        (goto _label Reset)))))

(event EventLaunchSwarmMissile
  (bind _returnvalue (+ 0.3 0.0))
  (bind _ship_data (Variables|Default|GetShip%20Data))
  (bind _ship_data_2 (Variables|Default|GetShip%20Data))
  (bind _ship_data_3 (Variables|Default|GetShip%20Data))
  (bind _ship_data_4 (Variables|Default|GetShip%20Data))
  (bind _ship_data_5 (Variables|Default|GetShip%20Data))
  (bind _swarmlauncher (Variables|Default|GetSwarmLauncher))
  ;[1 1 1] Swarm Missile System
  (Utilities|FlowControl|DoOnce false :!label _label
    (:Completed
      (Audio|PlaySoundatLocation "/Game/Assets/Audio/WAVs/MissileSwarmLaunch3_mixdown.MissileSwarmLaunch3_mixdown" (Transformation|GetWorldLocation (Variables|Character|GetMesh)) "0, 0, 0" 1.0 1.0 0.0 0 0 0 0)
      (Default|FireMissile (Variables|Default|GetAC_Weapons) (Variables|/Game/Assets/3D/Blueprints/Data_Assets/Ships/P_DataAsset_Ships.P_DataAsset_Ships_C|GetSwarm%20Missile%20Type _ship_data) _swarmlauncher (Variables|/Game/Assets/3D/Blueprints/Data_Assets/Ships/P_DataAsset_Ships.P_DataAsset_Ships_C|GetSwarm%20Missile%20Size _ship_data))
      (Utilities|FlowControl|Delay _returnvalue)
      (Default|FireMissile (Variables|Default|GetAC_Weapons) (Variables|/Game/Assets/3D/Blueprints/Data_Assets/Ships/P_DataAsset_Ships.P_DataAsset_Ships_C|GetSwarm%20Missile%20Type _ship_data_4) _swarmlauncher (Variables|/Game/Assets/3D/Blueprints/Data_Assets/Ships/P_DataAsset_Ships.P_DataAsset_Ships_C|GetSwarm%20Missile%20Size _ship_data_4))
      (Utilities|FlowControl|Delay _returnvalue)
      (Default|FireMissile (Variables|Default|GetAC_Weapons) (Variables|/Game/Assets/3D/Blueprints/Data_Assets/Ships/P_DataAsset_Ships.P_DataAsset_Ships_C|GetSwarm%20Missile%20Type _ship_data_3) _swarmlauncher (Variables|/Game/Assets/3D/Blueprints/Data_Assets/Ships/P_DataAsset_Ships.P_DataAsset_Ships_C|GetSwarm%20Missile%20Size _ship_data_3))
      (Utilities|FlowControl|Delay _returnvalue)
      (Default|FireMissile (Variables|Default|GetAC_Weapons) (Variables|/Game/Assets/3D/Blueprints/Data_Assets/Ships/P_DataAsset_Ships.P_DataAsset_Ships_C|GetSwarm%20Missile%20Type _ship_data_5) _swarmlauncher (Variables|/Game/Assets/3D/Blueprints/Data_Assets/Ships/P_DataAsset_Ships.P_DataAsset_Ships_C|GetSwarm%20Missile%20Size _ship_data_5))
      (Utilities|FlowControl|Delay _returnvalue)
      (Default|FireMissile (Variables|Default|GetAC_Weapons) (Variables|/Game/Assets/3D/Blueprints/Data_Assets/Ships/P_DataAsset_Ships.P_DataAsset_Ships_C|GetSwarm%20Missile%20Type _ship_data_2) _swarmlauncher (Variables|/Game/Assets/3D/Blueprints/Data_Assets/Ships/P_DataAsset_Ships.P_DataAsset_Ships_C|GetSwarm%20Missile%20Size _ship_data_2))
      (Utilities|FlowControl|Delay 15.0)
      (goto _label Reset))))

(event EventFireRailCannon
  ;[1 1 1] Weapons
  (Utilities|FlowControl|DoOnce false :!label _label
    (:Completed
      (Utilities|FlowControl|Delay (Variables|/Game/Assets/3D/Blueprints/Data_Assets/Weapons/P_DataAsset_Weapons.P_DataAsset_Weapons_C|GetInital%20Firing%20Delay (Variables|/Game/Assets/3D/Blueprints/Data_Assets/Ships/P_DataAsset_Ships.P_DataAsset_Ships_C|GetRail%20Cannon%20Projectile%20Type (Variables|Default|GetShip%20Data))))
      (Audio|PlaySoundatLocation "/Game/Assets/Audio/WAVs/RailCanon_Shot.RailCanon_Shot" (Transformation|GetActorLocation) "0, 0, 0" 1.0 1.0 0.0 0 0 0 0)
      (Default|FireCannon (Variables|Default|GetAC_Weapons) (Variables|/Game/Assets/3D/Blueprints/Data_Assets/Ships/P_DataAsset_Ships.P_DataAsset_Ships_C|GetRail%20Cannon%20Projectile%20Type (Variables|Default|GetShip%20Data)) (Variables|Default|GetRail%20Cannon))
      (Utilities|FlowControl|Delay (Variables|/Game/Assets/3D/Blueprints/Data_Assets/Weapons/P_DataAsset_Weapons.P_DataAsset_Weapons_C|GetDelay%20Between%20Rounds (Variables|/Game/Assets/3D/Blueprints/Data_Assets/Ships/P_DataAsset_Ships.P_DataAsset_Ships_C|GetRail%20Cannon%20Projectile%20Type (Variables|Default|GetShip%20Data))))
      (goto _label Reset))))

(event EventLaunchTorpedo
  (bind _ship_data (Variables|Default|GetShip%20Data))
  ;[1 1 1] Weapons
  (Utilities|FlowControl|DoOnce false :!label _label
    (:Completed
      (Default|FireMissile (Variables|Default|GetAC_Weapons) (Variables|/Game/Assets/3D/Blueprints/Data_Assets/Ships/P_DataAsset_Ships.P_DataAsset_Ships_C|GetTorpedo%20Type _ship_data) (Variables|Default|GetTorpedoLauncher) (Variables|/Game/Assets/3D/Blueprints/Data_Assets/Ships/P_DataAsset_Ships.P_DataAsset_Ships_C|GetTorpedo%20Size _ship_data))
      (Utilities|FlowControl|Delay 3e+01)
      (goto _label Reset))))

(fn ConstructionScript
  (|CallParentFunction))