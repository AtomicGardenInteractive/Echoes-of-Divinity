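; Base ship pawn for player and AI ships in a space RTS, configured from ShipData.
; BeginPlay spawns railgun and PDC turrets on named mesh sockets; Tick passes the current target to railguns and updates the health bar.
; Pawn sensing drives targeting: player ships follow Aggressive, Defensive or Recon stances, while AI ships approach and circle enemies.
; Bow, bridge and stern overlaps feed location-based damage; AnyDamage handles hull damage, retargeting and staged death explosions.
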(event EventBeginPlay
  (bind _self self)
  (bind _self_2 self)
  (Utilities|FlowControl|Sequence
    (:then_0
      ;[1 1 1] On Begin Play attaches Spawns and attaches Turrets to the Base Ship Mesh
      (for _array_element (Transformation|GetAllSocketNames (Variables|Default|GetShip%20Healthy%20Mesh))
        (if (Utilities|String|Contains (Utilities|String|ToString(Name) _array_element) "RailgunSocket")
          (bind _returnvalue (Game|SpawnActorfromClass (Variables|/Game/Assets/3D/Blueprints/Data_Assets/Ships/P_DataAsset_Ships.P_DataAsset_Ships_C|GetRailgunSocket%20Turret (Variables|Default|GetShip%20Data)) (Transformation|GetSocketTransform (Variables|Default|GetShip%20Healthy%20Mesh) _array_element "RTS_Component") "Undefined" _self_2 _self_2))
          (Transformation|AttachComponentToComponent _returnvalue (Variables|Default|GetShip%20Healthy%20Mesh) _array_element "SnapToTarget" "SnapToTarget" "SnapToTarget" true)
          (bind _asbp_turrets_p (Utilities|Casting|CastToBP_Turrets_P _returnvalue))
          (Utilities|Array|AddUnique (Variables|Default|GetMy%20Railgun%20Turrets) _asbp_turrets_p)
          (elif (Utilities|String|Contains (Utilities|String|ToString(Name) _array_element) "PDCSocket")
            (bind _returnvalue_2 (Game|SpawnActorfromClass (Variables|/Game/Assets/3D/Blueprints/Data_Assets/Ships/P_DataAsset_Ships.P_DataAsset_Ships_C|GetPDCSocket%20Turret (Variables|Default|GetShip%20Data)) (Transformation|GetSocketTransform (Variables|Default|GetShip%20Healthy%20Mesh) _array_element "RTS_Component") "Undefined" _self _self))
            (Transformation|AttachComponentToComponent _returnvalue_2 (Variables|Default|GetShip%20Healthy%20Mesh) _array_element "SnapToTarget" "SnapToTarget" "SnapToTarget" true)))))
    (:then_1
      ;[1 1 1] Sets Ships movement target indicator to hidden
      (Variables|Default|SetMovement%20Target%20Postions (Transformation|GetActorLocation))
      (Development|SetHiddeninGame (Variables|Default|GetHolo%20Ship%20Move%20Marker) true false))
    (:then_2
      (Rendering|SetCastShadow (Variables|Default|GetHealthbar) false))
    (:then_3
      (CameraFades|StartCameraFade :self (Game|GetPlayerCameraManager 0) :FromAlpha 1.0 :Duration 4.0 :bHoldWhenFinished true))))

(event OnComponentBeginOverlap(ShipHealthyMesh)
  (params (OverlappedComponent :type Primitive%20Component%20Object%20Reference) (OtherActor :type Actor%20Object%20Reference) (OtherComp :type Primitive%20Component%20Object%20Reference) (OtherBodyIndex :type Integer) (bFromSweep :type Boolean) (SweepResult :type Hit%20Result%20Structure%20%28by%20ref%29))
  ;[1 1 1] Hides Projectiles when they are in the ship
  (bind _asbp_bullet_p (Utilities|Casting|CastToBP_Bullet_P OtherActor))
  (Rendering|SetActorHiddenInGame _asbp_bullet_p false))

(event OnComponentBeginOverlap(Bridge)
  (params (OverlappedComponent :type Primitive%20Component%20Object%20Reference) (OtherActor :type Actor%20Object%20Reference) (OtherComp :type Primitive%20Component%20Object%20Reference) (OtherBodyIndex :type Integer) (bFromSweep :type Boolean) (SweepResult :type Hit%20Result%20Structure%20%28by%20ref%29))
  ;[1 1 1] Location Based Damage System
  (bind _asbp_bullet_p (Utilities|Casting|CastToBP_Bullet_P OtherActor))
  (Default|BridgeDamage (Variables|Default|GetShipHealth) (Variables|/Game/Assets/3D/Blueprints/Data_Assets/Bullets/P_DataAsset_Bullets.P_DataAsset_Bullets_C|GetProjectile%20Damage (Variables|/Game/Assets/3D/Blueprints/Projectiles/BP_Bullet_P.BP_Bullet_P_C|GetBullet%20Types _asbp_bullet_p))))

(event OnComponentBeginOverlap(Bow)
  (params (OverlappedComponent :type Primitive%20Component%20Object%20Reference) (OtherActor :type Actor%20Object%20Reference) (OtherComp :type Primitive%20Component%20Object%20Reference) (OtherBodyIndex :type Integer) (bFromSweep :type Boolean) (SweepResult :type Hit%20Result%20Structure%20%28by%20ref%29))
  ;[1 1 1] Location Based Damage System
  (bind _asbp_bullet_p (Utilities|Casting|CastToBP_Bullet_P OtherActor))
  (Default|BowDamage (Variables|Default|GetShipHealth) (Variables|/Game/Assets/3D/Blueprints/Data_Assets/Bullets/P_DataAsset_Bullets.P_DataAsset_Bullets_C|GetProjectile%20Damage (Variables|/Game/Assets/3D/Blueprints/Projectiles/BP_Bullet_P.BP_Bullet_P_C|GetBullet%20Types _asbp_bullet_p))))

(event OnComponentBeginOverlap(CapsuleComponent)
  (params (OverlappedComponent :type Primitive%20Component%20Object%20Reference) (OtherActor :type Actor%20Object%20Reference) (OtherComp :type Primitive%20Component%20Object%20Reference) (OtherBodyIndex :type Integer) (bFromSweep :type Boolean) (SweepResult :type Hit%20Result%20Structure%20%28by%20ref%29))
  ;[1 1 1] HealthUI Legacy Attempt for Reference
)

(event OnComponentBeginOverlap(Stern)
  (params (OverlappedComponent :type Primitive%20Component%20Object%20Reference) (OtherActor :type Actor%20Object%20Reference) (OtherComp :type Primitive%20Component%20Object%20Reference) (OtherBodyIndex :type Integer) (bFromSweep :type Boolean) (SweepResult :type Hit%20Result%20Structure%20%28by%20ref%29))
  ;[1 1 1] Location Based Damage System
  (bind _asbp_bullet_p (Utilities|Casting|CastToBP_Bullet_P OtherActor))
  (Default|SternDamage (Variables|Default|GetShipHealth) (Variables|/Game/Assets/3D/Blueprints/Data_Assets/Bullets/P_DataAsset_Bullets.P_DataAsset_Bullets_C|GetProjectile%20Damage (Variables|/Game/Assets/3D/Blueprints/Projectiles/BP_Bullet_P.BP_Bullet_P_C|GetBullet%20Types _asbp_bullet_p))))

(event OnComponentEndOverlap(ShipHealthyMesh)
  (params (OverlappedComponent :type Primitive%20Component%20Object%20Reference) (OtherActor :type Actor%20Object%20Reference) (OtherComp :type Primitive%20Component%20Object%20Reference) (OtherBodyIndex :type Integer))
  ;[1 1 1] Destroys actors on exit
  (Actor|DestroyActor OtherActor))

(event Game|Damage|EventAnyDamage
  (params (Damage :type Float%20%28single-precision%29) (DamageType :type Damage%20Type%20Object%20Reference) (InstigatedBy :type Controller%20Object%20Reference) (DamageCauser :type Actor%20Object%20Reference))
  (Utilities|FlowControl|Sequence
    (:then_0
      (Development|PrintString (Utilities|String|ToString(Float) (Variables|/Game/Assets/3D/Blueprints/ActorComponent/AC_ShipHealth.AC_ShipHealth_C|GetTotal%20Health%20Current (Variables|Default|GetShipHealth))))
      (bind (_is_dead _is_exploded) (Default|HullDamage (Variables|Default|GetShipHealth) Damage))
      ;[1 1 1] Checks to see if there is a local target on taking damage
      (Variables|Default|GetAttack%20Target
        (:then
          _)
        (:else
          (CallFunction|GetLocalTarget)
          (AI|AIMoveTo self "0, 0, 0" (Variables|Default|GetAttack%20Target) 1e+03 false
            (:then
              _))))
      ;[1 1 1] Ship Death Eitehr Explodes or Turns into debris
      (Utilities|FlowControl|Sequence
        (:then_0
          (if _is_dead
            ;[1 1 1] Sets Is Dead, Removes ship from selection, destroys all owned turrets and then self.
            (Variables|Default|SetIs%20Dead true)
            (bind _asplayer_controller_bp (Utilities|Casting|CastToPlayerController_BP (Game|GetPlayerController 0)))
            (Audio|PlaySoundatLocation "/Game/Assets/Audio/WAVs/CorvetteDestruction_mixdown.CorvetteDestruction_mixdown" (Transformation|GetWorldLocation (Variables|Character|GetMesh)) "0, 0, 0" 0.3 1.0 0.0 0 0 0 0)
            (Niagara|SpawnSystematLocation "/Game/Assets/3D/VFX/Niagara/BigExplosions/Niagara/NS_Air_1Modified.NS_Air_1Modified" (Transformation|GetWorldLocation (Variables|Default|GetBow)) "0, 0, 0" "0.100000,0.100000,0.100000")
            (Utilities|FlowControl|Delay 1.0)
            (Niagara|SpawnSystematLocation "/Game/Assets/3D/VFX/Niagara/BigExplosions/Niagara/NS_Air_1Modified.NS_Air_1Modified" (Transformation|GetWorldLocation (Variables|Default|GetStern)) "0, 0, 0" "0.100000,0.100000,0.100000")
            (Utilities|FlowControl|Delay 1.0)
            (Niagara|SpawnSystematLocation "/Game/Assets/3D/VFX/Niagara/BigExplosions/Niagara/NS_Air_1Modified.NS_Air_1Modified" (Transformation|GetWorldLocation (Variables|Default|GetBridge)) "0, 0, 0" "0.100000,0.100000,0.100000")
            (Utilities|FlowControl|Delay 2.0)
            (Niagara|SpawnSystematLocation "/Game/Assets/3D/VFX/Niagara/BigExplosions/Niagara/NS_Air_1.NS_Air_1" (Transformation|GetWorldLocation (Variables|Default|GetBridge)) "0, 0, 0" "0.300000,0.300000,0.300000")
            (Default|RemoveShip _asplayer_controller_bp self)
            (bind _arrayelement (Utilities|Array|ReverseforEachLoop (Actor|GetAttachedActors true false))
              (:LoopBody
                (Actor|DestroyActor _arrayelement))
              (:Completed
                (Actor|DestroyActor)))))
        (:then_1
          (if _is_exploded
            _))))))

(event OnSeePawn(PawnSensing)
  (params (Pawn :type Pawn%20Object%20Reference))
  ;[1 1 1] On Sensing Check if Ally
  (if (not (Actor|ActorHasTag Pawn (Variables|/Game/Assets/3D/Blueprints/Data_Assets/Ships/P_DataAsset_Ships.P_DataAsset_Ships_C|GetAlly%20Tag (Variables|Default|GetShip%20Data))))
    (switch Utilities|FlowControl|Switch|SwitchonEN_Ship_IsAI (Variables|/Game/Assets/3D/Blueprints/Data_Assets/Ships/P_DataAsset_Ships.P_DataAsset_Ships_C|GetIs%20Ai? (Variables|Default|GetShip%20Data))
      (:NewEnumerator0
        (if (Utilities|Operators|EqualEqual (Transformation|GetActorLocation self) (Variables|Default|GetMovement%20Target%20Postions) 5e+02)
          (switch Utilities|FlowControl|Switch|SwitchonEN_Ship_State (Variables|Default|GetEN%20Ship%20State)
            (:NewEnumerator11
              ;[1 1 1] Check is Target is still valid if not set new target and move towards
              (bind _attack_target (Variables|Default|GetAttack%20Target)
                (:then)
                (:else
                  (CallFunction|GetLocalTarget)
                  (bind _movementresult (AI|AIMoveTo self "0, 0, 0" _attack_target 2e+04 false)))))
            (:NewEnumerator12
              ;[1 1 1] Check if target is alive and if not get a new one
              (Variables|Default|GetAttack%20Target
                (:then)
                (:else
                  (CallFunction|GetLocalTarget))))
            (:NewEnumerator15
              ;[1 1 1] Flees
              (bind _outactors (Actor|GetAllActorswithTag "Home"))
              (AI|AIMoveTo 0 "0, 0, 0" (Utilities|Array|Get(acopy) _outactors) 2e+04 true)))))
      (:NewEnumerator3
        ;[1 1 1] Comp ships Targeting System
        (CallFunction|GetLocalTarget)
        (bind _attack_target_2 (Variables|Default|GetAttack%20Target)
          (:then
            (AI|AIMoveTo self "0, 0, 0" _attack_target_2 2e+04 false
              (:OnSuccess
                (Variables|Default|GetAttack%20Target
                  (:then
                    (CallFunction|ShipCircleTarget :!label _label)
                    (Utilities|FlowControl|Delay 0.0)
                    (goto _label))
                  (:else)))))
          (:else))))))

(event EventTick
  (params (DeltaSeconds :type Float%20%28single-precision%29))
  (Utilities|FlowControl|Sequence
    (:then_0
      (Rendering|Material|SetVectorParameterValue "/Game/Assets/3D/VFX/PostProcess/ShipPosition.ShipPosition" "ShipPosition" (Math|Conversions|ToLinearColor(Vector) (Transformation|GetActorLocation)) :!class /Script/Engine.KismetMaterialLibrary)
      ;[1 1 1] Sets move marker pos on tick
      (CallFunction|MovementTargetPostionMarker)
      (Variables|Default|GetAttack%20Target
        (:then
          ;[1 1 1] Sets Ship target to Turret targets
          (for _array_element (Variables|Default|GetMy%20Railgun%20Turrets)
            (Variables|/Game/Assets/3D/Blueprints/Turrets/BP_Turrets_P.BP_Turrets_P_C|SetOurTarget _array_element (Variables|Default|GetAttack%20Target))
            ;[1 1 1] Sound that plays once
            (switch Utilities|FlowControl|Switch|SwitchonEN_Ship_IsAI (Variables|/Game/Assets/3D/Blueprints/Data_Assets/Ships/P_DataAsset_Ships.P_DataAsset_Ships_C|GetIs%20Ai? (Variables|Default|GetShip%20Data))
              (:NewEnumerator0
                (Utilities|FlowControl|DoOnce false
                  (:Completed
                    (Audio|PlaySound2D "/Game/Assets/Audio/WAVs/VoiceLines/CorvetteVoiceLines/CorvetteEngagingTarget_mixdown.CorvetteEngagingTarget_mixdown" 2.0 1.0 0.0 0 0)))))))
        (:else
          (Utilities|FlowControl|DoOnce false) ; enters at Reset
        )))
    (:then_1
      ;[1 1 1] Display Health Bar Widget
      (bind _aswp_health_bar (Utilities|Casting|CastToWP_HealthBar (UserInterface|GetWidget (Variables|Default|GetHealthbar))))
      (Progress|SetPercent (Variables|/Game/Assets/UI/ShipUI/WP_HealthBar.WP_HealthBar_C|GetHealthBar _aswp_health_bar) (/ (Variables|/Game/Assets/3D/Blueprints/ActorComponent/AC_ShipHealth.AC_ShipHealth_C|GetTotal%20Health%20Current (Variables|Default|GetShipHealth)) (Variables|/Game/Assets/3D/Blueprints/Data_Assets/Ships/P_DataAsset_Ships.P_DataAsset_Ships_C|GetTotal%20Health%20Max (Variables|Default|GetShip%20Data))))
      (Transformation|SetWorldRotation (Variables|Default|GetHealthbar) (Math|Rotator|FindLookatRotation (Transformation|GetWorldLocation (Variables|Default|GetHealthbar)) (Transformation|GetWorldLocation (Variables|/Script/Engine.PlayerCameraManager|GetTransformComponent (Game|GetPlayerCameraManager 0)))) false false))))

(event Custom|Move%20Ship
  (params (Destination :type Vector) (Traget :type Actor%20Object%20Reference))
  (AI|AIMoveTo self Destination Traget 1e+03 false
    (:then
      (CallFunction|DisplayMoveMarker)
      ;[1 1 1] Only Allows sound to play once
      (Utilities|FlowControl|DoOnce false :!label _label
        (:Completed
          (Audio|PlaySound2D "/Game/Assets/Audio/WAVs/VoiceLines/CorvetteVoiceLines/CorvetteMovingToPosition_mixdown.CorvetteMovingToPosition_mixdown" 1.0 1.0 0.0 0 0)
          (Utilities|FlowControl|Delay 3.0)
          (goto _label Reset))))
    (:OnSuccess
      (CallFunction|HideMoveMarker))))

(fn ConstructionScript
  (bind _charactermovement (Variables|Character|GetCharacterMovement))
  (bind _ship_data (Variables|Default|GetShip%20Data))
  ;[1 1 1] Get Ship Type Info and Applies it
  (bind _ship_data_2 (Variables|Default|GetShip%20Data)
    (:then
      (Utilities|FlowControl|Sequence
        (:then_0
          (Components|StaticMesh|SetStaticMesh (Variables|Default|GetShip%20Damaged%20Mesh) (Variables|/Game/Assets/3D/Blueprints/Data_Assets/Ships/P_DataAsset_Ships.P_DataAsset_Ships_C|GetDamage%20Mesh _ship_data_2)))
        (:then_1
          (Components|StaticMesh|SetStaticMesh (Variables|Default|GetShip%20Healthy%20Mesh) (Variables|/Game/Assets/3D/Blueprints/Data_Assets/Ships/P_DataAsset_Ships.P_DataAsset_Ships_C|GetBase%20Mesh _ship_data_2)))
        (:then_2
          (Components|StaticMesh|SetStaticMesh (Variables|Default|GetHolo%20Ship%20Move%20Marker) (Variables|/Game/Assets/3D/Blueprints/Data_Assets/Ships/P_DataAsset_Ships.P_DataAsset_Ships_C|GetMovement%20Indicator%20Mesh _ship_data_2)))
        (:then_3
          (Default|SetUpHealth (Variables|Default|GetShipHealth) (Variables|Default|GetShip%20Data)))
        (:then_4
          (Variables|Default|SetTags (Variables|/Game/Assets/3D/Blueprints/Data_Assets/Ships/P_DataAsset_Ships.P_DataAsset_Ships_C|GetTags (Variables|Default|GetShip%20Data))))
        (:then_5
          (Variables|/Script/Engine.CharacterMovementComponent|SetMaxWalkSpeed _charactermovement (Variables|/Game/Assets/3D/Blueprints/Data_Assets/Ships/P_DataAsset_Ships.P_DataAsset_Ships_C|GetMovement%20Speed%20Max _ship_data))
          (Variables|/Script/Engine.CharacterMovementComponent|SetMaxAcceleration _charactermovement (Variables|/Game/Assets/3D/Blueprints/Data_Assets/Ships/P_DataAsset_Ships.P_DataAsset_Ships_C|GetMax%20Acceleration _ship_data))
          (Variables|/Script/Engine.CharacterMovementComponent|SetBrakingFrictionFactor _charactermovement (Variables|/Game/Assets/3D/Blueprints/Data_Assets/Ships/P_DataAsset_Ships.P_DataAsset_Ships_C|GetBraking%20Friction%20Factor _ship_data)))))
    (:else)))

(fn MovementTargetPostionMarker
  ;[1 1 1] Sets Move markers pos in World Space
  (Transformation|SetWorldLocation (Variables|Default|GetMovement%20Target%20Location) (Variables|Default|GetMovement%20Target%20Postions) false true))

(fn SelectionIndicatoron
  (bind _selction_indicator (Variables|Default|GetSelction%20Indicator))
  ;[1 1 1] Selection Circle
  (Development|SetHiddeninGame _selction_indicator false false)
  (Rendering|SetVisibility _selction_indicator true false)
  (if (not (Utilities|Operators|EqualEqual (Transformation|GetWorldLocation (Variables|Default|GetHolo%20Ship%20Move%20Marker)) (Transformation|GetWorldLocation (Variables|Character|GetMesh self)) 1e+04))
    (CallFunction|DisplayMoveMarker)))

(fn SelectionIndicatorOff
  (bind _selction_indicator (Variables|Default|GetSelction%20Indicator))
  ;[1 1 1] Selection Circle
  (Development|SetHiddeninGame _selction_indicator true false)
  (Rendering|SetVisibility _selction_indicator false false)
  (CallFunction|HideMoveMarker))

(fn DeathRattle
  ;[1 1 1] Sets Is Dead, Removes ship from selection, destroys all owned turrets and then self.
  (Variables|Default|SetIs%20Dead true)
  (bind _asplayer_controller_bp (Utilities|Casting|CastToPlayerController_BP (Game|GetPlayerController 0)))
  (Default|RemoveShip _asplayer_controller_bp self))

(fn CriticalDeathRattle
  ;[1 1 1] EXPLOSIONS
  (Actor|DestroyActor))

(fn SetShipState
  (params (EN%20Ship%20State :type EN_Ship_State%20Enum :default "NewEnumerator11"))
  (Variables|Default|SetEN%20Ship%20State EN%20Ship%20State))

(fn HideMoveMarker
  (bind _holo_ship_move_marker (Variables|Default|GetHolo%20Ship%20Move%20Marker))
  (Development|SetHiddeninGame _holo_ship_move_marker true false)
  (Rendering|SetVisibility _holo_ship_move_marker false false))

(fn DisplayMoveMarker
  (bind _holo_ship_move_marker (Variables|Default|GetHolo%20Ship%20Move%20Marker))
  (Development|SetHiddeninGame _holo_ship_move_marker false false)
  (Rendering|SetVisibility _holo_ship_move_marker true false))

(fn GetLocalTarget
  (bind _best_target (CallFunction|BestTarget self (Variables|/Game/Assets/3D/Blueprints/Data_Assets/Ships/P_DataAsset_Ships.P_DataAsset_Ships_C|GetAlly%20Tag (Variables|Default|GetShip%20Data))))
  (Variables|Default|SetAttack%20Target _best_target))

(fn ShipCircleTarget
  (bind _attack_target (Variables|Default|GetAttack%20Target))
  (Utilities|IsValid _attack_target
    (:Is%20Valid
      (Pawn|Input|AddMovementInput self (Transformation|GetActorRightVector _attack_target) 1.0 false))))