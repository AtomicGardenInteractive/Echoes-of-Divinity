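; Test ship Blueprint for a selectable unit with weapons, health and a move-target marker.
; Cruise and swarm events spawn homing missiles at the missile port, singly or as a delayed five-shot volley; FireGun spawns bullets, while rail weapon events only play sound.
; Damage lowers clamped health; at zero the ship deregisters from the player controller and destroys itself.
; Tick pins the marker to TargetPosition, and selection functions toggle it with the selection circle.
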(event Custom|Fire%20Gun
  (params (Spawn%20Transform%20Scale :type Vector))
  (bind _self self)
  (bind _bullet_spawn (Variables|Default|GetBullet%20Spawn))
  (bind _returnvalue (Transformation|GetWorldTransform _bullet_spawn))
  ;[1 1 1] Fire Gun
  (bind _returnvalue_2 (Game|SpawnActorfromClass "/Game/Assets/3D/Blueprints/Tests/Test_Bullet_BP.Test_Bullet_BP_C" (Math|Transform|MakeTransform (.location _returnvalue) (.rotation _returnvalue) Spawn%20Transform%20Scale) "AlwaysSpawn" _self _self))
  (Development|PrintString (Utilities|GetDisplayName _returnvalue_2)))

(event Custom|Fire%20Missile
  (params (Missile%20Size :type Vector))
  (bind _missileport (Variables|Default|GetMissilePort))
  (bind _returnvalue (Transformation|GetWorldTransform _missileport))
  ;[1 1 1] Fire Homing Missile
  (Game|SpawnActorfromClass "/Game/Assets/3D/Blueprints/Tests/Test_Missile_BP.Test_Missile_BP_C" (Math|Transform|MakeTransform (.location _returnvalue) (.rotation _returnvalue) Missile%20Size) "AlwaysSpawn" self 0))

(event Custom|Rail%20Cannon
  ;[1 1 1] Rail Cannon Fire
  (Audio|PlaySoundatLocation 0 (Transformation|GetActorLocation) "0, 0, 0" 1.0 1.0 0.0 0 0 0 0)
  (Utilities|FlowControl|Delay 0.75))

(event Custom|Rail%20Gun
  ;[1 1 1] Rail Gun Fire
  (Audio|PlaySoundatLocation 0 (Transformation|GetActorLocation) "0, 0, 0" 1.0 1.0 0.0 0 0 0 0))

(event Custom|Swarm%20Missiles
  (bind _swarm_size (Variables|Default|GetSwarm%20Size))
  (bind _swarm_launch_delay (Variables|Default|GetSwarm%20Launch%20Delay))
  ;[1 1 1] Swarm Missiles Launch
  (Audio|PlaySoundatLocation 0 (Transformation|GetActorLocation) "0, 0, 0" 1.0 1.0 0.0 0 0 0 0)
  (CallFunction|FireMissile _swarm_size)
  (Utilities|FlowControl|Delay _swarm_launch_delay)
  (CallFunction|FireMissile _swarm_size)
  (Utilities|FlowControl|Delay _swarm_launch_delay)
  (CallFunction|FireMissile _swarm_size)
  (Utilities|FlowControl|Delay _swarm_launch_delay)
  (CallFunction|FireMissile _swarm_size)
  (Utilities|FlowControl|Delay _swarm_launch_delay)
  (CallFunction|FireMissile _swarm_size))

(event Custom|Cruise%20Missile
  ;[1 1 1] Launch Cruise Missile
  (Audio|PlaySoundatLocation 0 (Transformation|GetActorLocation) "0, 0, 0" 1.0 1.0 0.0 0 0 0 0)
  (Utilities|FlowControl|Delay 0.75)
  (CallFunction|FireMissile (Variables|Default|GetMissile%20Size)))

(event Custom|Server%20Fire%20Missile
  (params (Missile%20Size :type Vector))
  (CallFunction|FireMissile Missile%20Size))

(event EventBeginPlay
  ;[1 1 1] Nav Target
  (Variables|Default|SetTarget%20Position (Pawn|GetNavAgentLocation)))

(event EventTick
  (params (DeltaSeconds :type Float%20%28single-precision%29))
  ;[1 1 1] Nav Target
  (Transformation|SetWorldLocation (Variables|Default|GetMovementMakerLocation) (Variables|Default|GetTarget%20Position) false true))

(event Game|Damage|EventAnyDamage
  (params (Damage :type Float%20%28single-precision%29) (DamageType :type Damage%20Type%20Object%20Reference) (InstigatedBy :type Controller%20Object%20Reference) (DamageCauser :type Actor%20Object%20Reference))
  ;[1 1 1] Damage System
  (if (not (Variables|Default|GetIsDead))
    (bind _output_get (Variables|Default|SetCurrent%20Health (Math|Float|Clamp(Float) (- (Variables|Default|GetCurrent%20Health) Damage) 0.0 (Variables|Default|GetMax%20Health))))
    (Development|PrintString (Utilities|String|ToString(Float) _output_get) true true "(R=0.054480,G=0.863157,B=0.045186,A=1.000000)")
    (if (== _output_get 0.0)
      (bind _asplayer_controller_bp (Utilities|Casting|CastToPlayerController_BP (Game|GetPlayerController 0)))
      (Default|RemoveShip _asplayer_controller_bp self)
      (Variables|Default|SetIsDead true)
      (Actor|DestroyActor))))

(fn ConstructionScript)

(fn SelectionIndicatoron
  (bind _sphere (Variables|Default|GetSphere))
  (bind _selction_indicator (Variables|Default|GetSelction%20Indicator))
  ;[1 1 1] Selection Circle
  (Development|SetHiddeninGame _selction_indicator false false)
  (Rendering|SetVisibility _selction_indicator true false)
  ;[1 1 1] Move Marker
  (Development|SetHiddeninGame _sphere false false)
  (Rendering|SetVisibility _sphere true false))

(fn SelectionIndicatorOff
  (bind _sphere (Variables|Default|GetSphere))
  (bind _selction_indicator (Variables|Default|GetSelction%20Indicator))
  ;[1 1 1] Selection Circle
  (Development|SetHiddeninGame _selction_indicator true false)
  (Rendering|SetVisibility _selction_indicator false false)
  ;[1 1 1] Move Marker
  (Development|SetHiddeninGame _sphere true false)
  (Rendering|SetVisibility _sphere false false))