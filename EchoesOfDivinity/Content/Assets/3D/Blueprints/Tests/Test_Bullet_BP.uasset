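; Test projectile actor for bullets, configured by a BulletTypes data reference.
; The construction script sets mesh, lifespan and initial projectile speed from that data when it is valid.
; On overlap with any actor other than its owner, it applies the configured damage with the owner as causer.
; Debug printing and destroy-on-hit logic for rail gun slugs are disconnected, so overlaps never destroy the bullet.
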(event Collision|EventActorBeginOverlap
  (params (OtherActor :type Actor%20Object%20Reference))
  (bind _returnvalue (Components|GetOwner))
  (if (not (== OtherActor _returnvalue))
    (bind _returnvalue_2 (Game|Damage|ApplyDamage OtherActor (Variables|/Game/Assets/3D/Blueprints/Data_Assets/Bullets/P_DataAsset_Bullets.P_DataAsset_Bullets_C|GetProjectile%20Damage (Variables|Default|GetBullet%20Types)) 0 _returnvalue))))

(fn ConstructionScript
  (bind _bullet_types (Variables|Default|GetBullet%20Types)
    (:then
      (Utilities|FlowControl|Sequence
        (:then_0
          (Components|StaticMesh|SetStaticMesh (Variables|Default|GetStaticMesh) (Variables|/Game/Assets/3D/Blueprints/Data_Assets/Bullets/P_DataAsset_Bullets.P_DataAsset_Bullets_C|GetBullet%20Mesh _bullet_types)))
        (:then_1
          (Actor|SetLifeSpan (Variables|/Game/Assets/3D/Blueprints/Data_Assets/Bullets/P_DataAsset_Bullets.P_DataAsset_Bullets_C|GetProjectile%20Range%20%28Life%20Span%29 _bullet_types)))
        (:then_2
          (Variables|/Script/Engine.ProjectileMovementComponent|SetInitialSpeed (Variables|Default|GetProjectileMovement) (Variables|/Game/Assets/3D/Blueprints/Data_Assets/Bullets/P_DataAsset_Bullets.P_DataAsset_Bullets_C|GetProjectile%20Speed _bullet_types)))))
    (:else)))