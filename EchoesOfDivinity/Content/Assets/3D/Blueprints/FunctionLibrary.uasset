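; Blueprint function library for picking a ship's target, with a line-of-sight helper.
; Best Target sphere-overlaps BP_Ship_P actors within SensingRange, excluding those with the given tag, and keeps the closest one visible to the caller.
; HasLineOfSight runs a debug-drawn Visibility trace, ignoring both caller and candidate, and counts no hit as clear sight.
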(fn HasLineOfSight
  (params (From :type Vector) (To :type Vector) (ActorsToIgnore :type Array%20of%20Actor%20Object%20References))
  (bind _returnvalue (Collision|LineTraceByChannel 0 From To "TraceTypeQuery1" false ActorsToIgnore "ForOneFrame" false "(R=1.000000,G=0.000000,B=0.000000,A=1.000000)" "(R=0.000000,G=1.000000,B=0.000000,A=1.000000)" 1.0))
  (return (not _returnvalue)))

(fn BestTarget
  (params (Ref%20to%20Self :type Actor%20Object%20Reference) (Tag%20To%20Ignore :type Name))
  (LocalVariables|SetBestDistance%28Local%29 (+ 1.0 (LocalVariables|GetSensingRange)))
  (bind _outactors (Actor|GetAllActorswithTag Ref%20to%20Self Tag%20To%20Ignore))
  (bind _outactors_2 (Collision|SphereOverlapActors Ref%20to%20Self (Transformation|GetActorLocation Ref%20to%20Self) (LocalVariables|GetSensingRange) (Utilities|Array|MakeArray "ObjectTypeQuery8") "/Game/Assets/3D/Blueprints/BP_Ship_P.BP_Ship_P_C" _outactors))
  (for _array_element _outactors_2
    (bind _output_get (LocalVariables|SetCurrentTarget%28Local%29 _array_element))
    (bind _output_get_2 (LocalVariables|SetCurrentDistance%28Local%29 (Transformation|GetDistanceTo _output_get Ref%20to%20Self)))
    (if (or (< _output_get_2 (LocalVariables|GetBestDistance%28Local%29)) (not (Utilities|IsValid (LocalVariables|GetBestTarget%28Local%29))))
      (bind _result (CallFunction|HasLineOfSight (Transformation|GetWorldLocation (Variables|/Script/Engine.Actor|GetRootComponent Ref%20to%20Self)) (Transformation|GetActorLocation (LocalVariables|GetCurrentTarget%28Local%29)) (Utilities|Array|MakeArray Ref%20to%20Self (LocalVariables|GetCurrentTarget%28Local%29)) Ref%20to%20Self))
      (if _result
        (LocalVariables|SetBestTarget%28Local%29 (LocalVariables|GetCurrentTarget%28Local%29))
        (LocalVariables|SetBestDistance%28Local%29 (LocalVariables|GetCurrentDistance%28Local%29)))))
  (bind _output_get_3 (LocalVariables|SetOurTarget (LocalVariables|GetBestTarget%28Local%29)))
  (Utilities|IsValid _output_get_3
    (:Is%20Valid
      (return _output_get_3))))