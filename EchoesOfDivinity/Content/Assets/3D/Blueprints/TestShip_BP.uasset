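; Selectable ship actor with health, two rail weapons and indicators for selection and movement target.
; RailCannon fires one delayed slug and RailGun a timed five-shot burst, both spawning Bullet_BP at BulletSpawn with their own slug scale.
; Damage lowers clamped health; at zero the ship removes itself from PlayerController_BP and is destroyed.
; Tick pins the move marker to TargetPostion, while selection functions toggle the circle and marker.
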(event Custom|Fire%20Gun
  (params (Spawn%20Transform%20Scale :type Vector))
  (bind _bullet_spawn (Variables|Default|GetBullet%20Spawn))
  (bind _returnvalue (Transformation|GetWorldTransform _bullet_spawn))
  ;[1 1 1] Fire Gun
  (Game|SpawnActorfromClass "/Game/Assets/3D/Blueprints/Bullet_BP.Bullet_BP_C" (Math|Transform|MakeTransform (.location _returnvalue) (.rotation _returnvalue) Spawn%20Transform%20Scale) "AlwaysSpawn" self 0))

(event Custom|Rail%20Cannon
  ;[1 1 1] Rail Cannon Fire
  (Audio|PlaySoundatLocation "/Game/Assets/Audio/TempTobeDeleted/Rail_Cannon_Cue.Rail_Cannon_Cue" (Transformation|GetActorLocation) "0, 0, 0" 1.0 1.0 0.0 0 0 0 0)
  (Utilities|FlowControl|Delay 0.75)
  (CallFunction|FireGun (Variables|Default|GetRail%20Cannon%20Slug%20Size)))

(event Custom|Rail%20Gun
  (bind _rail_gun_slug_size (Variables|Default|GetRail%20Gun%20Slug%20Size))
  ;[1 1 1] Rail Gun Fire
  (Audio|PlaySoundatLocation 0 (Transformation|GetActorLocation) "0, 0, 0" 1.0 1.0 0.0 0 0 0 0)
  (Utilities|FlowControl|Delay 0.025)
  (CallFunction|FireGun _rail_gun_slug_size)
  (Utilities|FlowControl|Delay 0.025)
  (CallFunction|FireGun _rail_gun_slug_size)
  (Utilities|FlowControl|Delay 0.025)
  (CallFunction|FireGun _rail_gun_slug_size)
  (Utilities|FlowControl|Delay 0.025)
  (CallFunction|FireGun _rail_gun_slug_size)
  (Utilities|FlowControl|Delay 0.025)
  (CallFunction|FireGun _rail_gun_slug_size))

(event EventBeginPlay
  (Variables|Default|SetTarget%20Postion (Pawn|GetNavAgentLocation)))

(event Collision|EventActorBeginOverlap
  (params (OtherActor :type Actor%20Object%20Reference)))

(event EventTick
  (params (DeltaSeconds :type Float%20%28single-precision%29))
  (Transformation|SetWorldLocation (Variables|Default|GetMovementMakerLocation) (Variables|Default|GetTarget%20Postion) false true))

(event Game|Damage|EventAnyDamage
  (params (Damage :type Float%20%28single-precision%29) (DamageType :type Damage%20Type%20Object%20Reference) (InstigatedBy :type Controller%20Object%20Reference) (DamageCauser :type Actor%20Object%20Reference))
  ;[1 1 1] Damage System
  (if (not (Variables|Default|GetIsDead))
    (bind _output_get (Variables|Default|SetCurrent%20Health (Math|Float|Clamp(Float) (- (Variables|Default|GetCurrent%20Health) Damage) 0.0 (Variables|Default|GetMax%20Health))))
    (Development|PrintString (Utilities|String|ToString(Float) _output_get) true true "(R=0.054480,G=0.863157,B=0.045186,A=1.000000)")
    (if (== _output_get 0.0)
      (bind _asplayer_controller_bp (Utilities|Casting|CastToPlayerController_BP (Game|GetPlayerController 0)))
      (Default|RemoveShip _asplayer_controller_bp self)
      (Variables|Default|SetIsDead true)
      (Actor|DestroyActor))))

(fn ConstructionScript)

(fn SelectionIndicatoron
  (bind _sphere (Variables|Default|GetSphere))
  (bind _selction_indicator (Variables|Default|GetSelction%20Indicator))
  ;[1 1 1] Selection Circle
  (Development|SetHiddeninGame _selction_indicator false false)
  (Rendering|SetVisibility _selction_indicator true false)
  ;[1 1 1] Move Marker
  (Development|SetHiddeninGame _sphere false false)
  (Rendering|SetVisibility _sphere true false))

(fn SelectionIndicatorOff
  (bind _sphere (Variables|Default|GetSphere))
  (bind _selction_indicator (Variables|Default|GetSelction%20Indicator))
  ;[1 1 1] Selection Circle
  (Development|SetHiddeninGame _selction_indicator true false)
  (Rendering|SetVisibility _selction_indicator false false)
  ;[1 1 1] Move Marker
  (Development|SetHiddeninGame _sphere true false)
  (Rendering|SetVisibility _sphere false false))