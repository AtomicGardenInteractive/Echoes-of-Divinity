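; TestShip is a clickable ship actor that can be selected and deselected.
; Clicking it fires ShipSelected, which registers the ship in PlayerController_BP's selected list and shows a decal as the selection indicator.
; A DeselectShip event reverses this, removing the ship from the controller and hiding the decal.
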(event Custom|Ship%20Selected
  (CallFunction|AddShiptoSelection))

(event EventBeginPlay)

(event Collision|EventActorBeginOverlap
  (params (OtherActor :type Actor%20Object%20Reference)))

(event EventTick
  (params (DeltaSeconds :type Float%20%28single-precision%29)))

(event MouseInput|EventActorOnClicked
  (params (ButtonPressed :type Key%20Structure :default "None"))
  (CallFunction|ShipSelected))

(event EventDeselectShip
  (CallFunction|RemoveShipfromSelection))

(fn ConstructionScript)

(fn SelectionIndicatoron
  (bind _decal (Variables|Default|GetDecal))
  (Development|SetHiddeninGame _decal false false)
  (Rendering|SetVisibility _decal true false))

(fn SelectionIndicatorOff
  (bind _decal (Variables|Default|GetDecal))
  (Development|SetHiddeninGame _decal true false)
  (Rendering|SetVisibility _decal false false))

(fn RemoveShipfromSelection
  (Utilities|FlowControl|Sequence
    (:then_0
      (bind _asplayer_controller_bp (Utilities|Casting|CastToPlayerController_BP (Game|GetPlayerController 0)))
      (Default|RemoveShip _asplayer_controller_bp self))
    (:then_1
      (CallFunction|SelectionIndicatorOff))))

(fn AddShiptoSelection
  (Utilities|FlowControl|Sequence
    (:then_0
      (bind _asplayer_controller_bp (Utilities|Casting|CastToPlayerController_BP (Game|GetPlayerController 0)))
      (Default|AddShiptoSelectedList _asplayer_controller_bp self))
    (:then_1
      (CallFunction|SelectionIndicatoron))))