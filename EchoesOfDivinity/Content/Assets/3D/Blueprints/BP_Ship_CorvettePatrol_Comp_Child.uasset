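; Child Blueprint of a patrol corvette ship that chases the SplinePawn_BP pawn once it sees it.
; PawnSensing's OnSeePawn passes a DoOnce gate, then casts the seen pawn and issues an AI MoveTo toward it with near-zero acceptance radius.
; The gate resets only when the move succeeds, so a failed cast or move leaves it closed.
; Construction defers to the parent.
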(event OnSeePawn(PawnSensing)
  (params (Pawn :type Pawn%20Object%20Reference))
  (Utilities|FlowControl|DoOnce false :!label _label
    (:Completed
      (bind _asspline_pawn_bp (Utilities|Casting|CastToSplinePawn_BP Pawn))
      (AI|AIMoveTo self "0, 0, 0" _asspline_pawn_bp 0.0001 false
        (:OnSuccess
          (goto _label Reset))))))

(event EventBeginPlay
  (|CallParentFunction) ; This node is disabled and will not be called.\nDrag off pins to build functionality.
)

(event Collision|EventActorBeginOverlap
  (params (OtherActor :type Actor%20Object%20Reference))
  (|CallParentFunction OtherActor) ; This node is disabled and will not be called.\nDrag off pins to build functionality.
)

(event EventTick
  (params (DeltaSeconds :type Float%20%28single-precision%29))
  (|CallParentFunction DeltaSeconds) ; This node is disabled and will not be called.\nDrag off pins to build functionality.
)

(fn ConstructionScript
  (|CallParentFunction))