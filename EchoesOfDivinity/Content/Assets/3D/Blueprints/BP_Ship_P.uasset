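; BP_Ship_P is a ship actor configured from ShipData, with sectional hit volumes and unfinished damage handling.
; The construction script applies ShipData's healthy and damaged meshes and collects the healthy mesh's socket names into GunSockets.
; Stern, Bridge and Bow overlaps unhide the other actor, while leaving the Hull volume destroys it.
; ShipHealth's per-section damage calls are present but unconnected, so overlaps apply no damage.
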(event EventBeginPlay)

(event Collision|EventActorBeginOverlap
  (params (OtherActor :type Actor%20Object%20Reference)))

(event EventTick
  (params (DeltaSeconds :type Float%20%28single-precision%29)))

(event OnComponentBeginOverlap(Stern)
  (params (OverlappedComponent :type Primitive%20Component%20Object%20Reference) (OtherActor :type Actor%20Object%20Reference) (OtherComp :type Primitive%20Component%20Object%20Reference) (OtherBodyIndex :type Integer) (bFromSweep :type Boolean) (SweepResult :type Hit%20Result%20Structure%20%28by%20ref%29))
  (Rendering|SetActorHiddenInGame OtherActor false))

(event OnComponentBeginOverlap(Bridge)
  (params (OverlappedComponent :type Primitive%20Component%20Object%20Reference) (OtherActor :type Actor%20Object%20Reference) (OtherComp :type Primitive%20Component%20Object%20Reference) (OtherBodyIndex :type Integer) (bFromSweep :type Boolean) (SweepResult :type Hit%20Result%20Structure%20%28by%20ref%29))
  (Rendering|SetActorHiddenInGame OtherActor false))

(event OnComponentBeginOverlap(Bow)
  (params (OverlappedComponent :type Primitive%20Component%20Object%20Reference) (OtherActor :type Actor%20Object%20Reference) (OtherComp :type Primitive%20Component%20Object%20Reference) (OtherBodyIndex :type Integer) (bFromSweep :type Boolean) (SweepResult :type Hit%20Result%20Structure%20%28by%20ref%29))
  (Rendering|SetActorHiddenInGame OtherActor false))

(event OnComponentBeginOverlap(Hull)
  (params (OverlappedComponent :type Primitive%20Component%20Object%20Reference) (OtherActor :type Actor%20Object%20Reference) (OtherComp :type Primitive%20Component%20Object%20Reference) (OtherBodyIndex :type Integer) (bFromSweep :type Boolean) (SweepResult :type Hit%20Result%20Structure%20%28by%20ref%29)))

(event OnComponentEndOverlap(Hull)
  (params (OverlappedComponent :type Primitive%20Component%20Object%20Reference) (OtherActor :type Actor%20Object%20Reference) (OtherComp :type Primitive%20Component%20Object%20Reference) (OtherBodyIndex :type Integer))
  (Actor|DestroyActor OtherActor))

(fn ConstructionScript
  (bind _ship_data (Variables|Default|GetShip%20Data)
    (:then
      (Utilities|FlowControl|Sequence
        (:then_0
          (Components|StaticMesh|SetStaticMesh (Variables|Default|GetShip%20Damaged%20Mesh) (Variables|/Game/Assets/3D/Blueprints/Data_Assets/Ships/P_DataAsset_Ships.P_DataAsset_Ships_C|GetDamage%20Mesh _ship_data)))
        (:then_1
          (Components|StaticMesh|SetStaticMesh (Variables|Default|GetShip%20Healthy%20Mesh) (Variables|/Game/Assets/3D/Blueprints/Data_Assets/Ships/P_DataAsset_Ships.P_DataAsset_Ships_C|GetBase%20Mesh _ship_data)))
        (:then_2
          ;[1 0 0] TERRIBLE NEEDS HELP
          (for _array_element (Transformation|GetAllSocketNames (Variables|Default|GetShip%20Healthy%20Mesh))
            (Utilities|Array|AddUnique (Variables|Default|GetGun%20Sockets) _array_element)))))
    (:else)))