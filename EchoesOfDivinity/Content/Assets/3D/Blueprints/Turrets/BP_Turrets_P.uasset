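; Data-driven turret that takes its meshes, projectile and fire timing from TurretType and copies its owner's tags.
; Only Point Defense Gun types acquire targets here, picking the nearest visible missile within range via sphere overlap, ignoring actors sharing the first tag.
; With a valid target, Tick turns the gun at constant speed and runs a DoOnce-and-Delay firing loop with random jitter, spawning projectile, effect and sound.
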(event EventTick
  (params (DeltaSeconds :type Float%20%28single-precision%29))
  (bind _arrow (Variables|Default|GetArrow))
  (bind _turret_type (Variables|Default|GetTurret%20Type))
  (bind _returnvalue (Transformation|GetWorldTransform _arrow))
  (switch Utilities|FlowControl|Switch|SwitchonEN_Weapons_Types (Variables|/Game/Assets/3D/Blueprints/Data_Assets/Weapons/P_DataAsset_Weapons.P_DataAsset_Weapons_C|GetWeapon%20Type (Variables|Default|GetTurret%20Type))
    (:NewEnumerator0
      _)
    (:NewEnumerator1
      _)
    (:NewEnumerator2
      _)
    (:NewEnumerator3
      (Private|FIndBestTargetMissile (Utilities|Array|Get(acopy) (Variables|Actor|GetTags)))))
  (Variables|Default|GetOurTarget
    (:then
      (Private|UpdateTurretRotation DeltaSeconds)
      (Utilities|FlowControl|DoOnce false :!label _label
        (:Completed
          (Utilities|FlowControl|Delay (Variables|/Game/Assets/3D/Blueprints/Data_Assets/Weapons/P_DataAsset_Weapons.P_DataAsset_Weapons_C|GetInital%20Firing%20Delay _turret_type))
          (Utilities|FlowControl|Delay (Math|Random|RandomFloatinRange 0.0 0.2))
          (Game|SpawnActorfromClass (Variables|/Game/Assets/3D/Blueprints/Data_Assets/Weapons/P_DataAsset_Weapons.P_DataAsset_Weapons_C|GetProjectile _turret_type) (Math|Transform|MakeTransform (.location _returnvalue) (.rotation _returnvalue) (Variables|/Game/Assets/3D/Blueprints/Data_Assets/Weapons/P_DataAsset_Weapons.P_DataAsset_Weapons_C|GetProjectile%20Size _turret_type)) "AlwaysSpawn" self 0)
          (Niagara|SpawnSystematLocation 0 (.location _returnvalue) (.rotation _returnvalue))
          (Audio|PlaySoundatLocation "/Game/Assets/Audio/WAVs/RailgunFire2_mixdown.RailgunFire2_mixdown" (.location _returnvalue) "0, 0, 0" 1.0 1.0 0.0 0 0 0 0)
          (Utilities|FlowControl|Delay (Variables|/Game/Assets/3D/Blueprints/Data_Assets/Weapons/P_DataAsset_Weapons.P_DataAsset_Weapons_C|GetDelay%20Between%20Rounds (Variables|Default|GetTurret%20Type)))
          (goto _label Reset))))
    (:else)))

(fn ConstructionScript
  (bind _turret_type (Variables|Default|GetTurret%20Type)
    (:then
      (Utilities|FlowControl|Sequence
        (:then_0
          (Components|StaticMesh|SetStaticMesh (Variables|Default|GetTurret) (Variables|/Game/Assets/3D/Blueprints/Data_Assets/Weapons/P_DataAsset_Weapons.P_DataAsset_Weapons_C|GetGun%20Mesh _turret_type)))
        (:then_1
          (Components|StaticMesh|SetStaticMesh (Variables|Default|GetBase) (Variables|/Game/Assets/3D/Blueprints/Data_Assets/Weapons/P_DataAsset_Weapons.P_DataAsset_Weapons_C|GetMount%20Mesh _turret_type)))
        (:then_2
          (Variables|Default|SetTags (Variables|/Script/Engine.Actor|GetTags (Components|GetOwner))))))
    (:else)))

(fn FIndBestTargetMissile
  (params (Tag%20to%20Ignore :type Name))
  (LocalVariables|SetBestDistance%28Local%29 (+ (Variables|Constant|GetSensingRange) 1.0))
  (bind _outactors (Actor|GetAllActorswithTag Tag%20to%20Ignore))
  (bind _outactors_2 (Collision|SphereOverlapActors (Transformation|GetActorLocation) (Variables|Constant|GetSensingRange) (Utilities|Array|MakeArray "ObjectTypeQuery10") "/Script/Engine.Actor" _outactors))
  (for _array_element _outactors_2
    (bind _output_get (LocalVariables|SetCurrentTarget%28Local%29 _array_element))
    (bind _output_get_2 (LocalVariables|SetCurrentDistance%28Local%29 (Transformation|GetDistanceTo _output_get self)))
    (if (or (< _output_get_2 (LocalVariables|GetBestDistance%28Local%29)) (not (Utilities|IsValid (LocalVariables|GetBestTarget%28Local%29))))
      (bind _result (CallFunction|HasLineOfSight (Transformation|GetWorldLocation (Variables|Default|GetArrow)) (Transformation|GetActorLocation (LocalVariables|GetCurrentTarget%28Local%29)) (Utilities|Array|MakeArray self (LocalVariables|GetCurrentTarget%28Local%29))))
      (if _result
        (LocalVariables|SetBestTarget%28Local%29 (LocalVariables|GetCurrentTarget%28Local%29))
        (LocalVariables|SetBestDistance%28Local%29 (LocalVariables|GetCurrentDistance%28Local%29)))))
  (Variables|Default|SetOurTarget (LocalVariables|GetBestTarget%28Local%29)))

(fn UpdateTurretRotation
  (params (DeltaSeconds :type Float%20%28double-precision%29))
  (Transformation|SetWorldRotation (Variables|Default|GetTurret) (Class|KismetMathLibrary|RInterptoConstant (Transformation|GetWorldRotation (Variables|Default|GetTurret)) (Math|Rotator|FindLookatRotation (Transformation|GetWorldLocation (Variables|Default|GetTurret)) (Transformation|GetActorLocation (Variables|Default|GetOurTarget))) DeltaSeconds (Variables|Constant|GetRotation%20Speed)) false false))