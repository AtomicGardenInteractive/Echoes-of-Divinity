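; BP_VoiceCollsion_Scanners_Probes is a trigger actor that delivers a one-time voice-over and on-screen prompt about scanners and probes.
; When a BP_Ship_Destroyer overlaps it, a DoOnce adds the WP_ProbeUsage widget and plays the Whitlock scanner line.
; Delays sequence the AI short-range probe line afterward, then remove the widget.
; Casts for other ship classes and a debug print remain in the graph but never run.
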(event EventBeginPlay
  (|CallParentFunction) ; This node is disabled and will not be called.\nDrag off pins to build functionality.
)

(event Collision|EventActorBeginOverlap
  (params (OtherActor :type Actor%20Object%20Reference))
  (Utilities|Casting|CastToBP_Ship_Destroyer OtherActor)
  (Utilities|FlowControl|DoOnce false
    (:Completed
      (bind _returnvalue (UserInterface|CreateWidget "/Game/Assets/UI/OnboardingLevel/WP_ProbeUsage.WP_ProbeUsage_C"))
      (UserInterface|Viewport|AddtoViewport _returnvalue 0)
      (Audio|PlaySound2D "/Game/Assets/Audio/WAVs/VoiceLines/CmdrWhitlock/WhitlockScanners_mixdown.WhitlockScanners_mixdown" 1.0 1.0 0.0 0 0 false)
      (Utilities|FlowControl|Delay 5.0)
      (Audio|PlaySound2D "/Game/Assets/Audio/WAVs/VoiceLines/ShipAI/AIShortRangeProbes_mixdown.AIShortRangeProbes_mixdown" 1.0 1.0 0.0 0 0)
      (Utilities|FlowControl|Delay 2e+01)
      (Widget|RemovefromParent _returnvalue))))

(event EventTick
  (params (DeltaSeconds :type Float%20%28single-precision%29))
  (|CallParentFunction DeltaSeconds) ; This node is disabled and will not be called.\nDrag off pins to build functionality.
)

(fn ConstructionScript
  (|CallParentFunction))