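; A trigger actor that plays ship AI voice lines about the corvette station being gone when the destroyer ship enters it.
; On the first overlap by BP_Ship_Destroyer, a DoOnce adds the WP_HendrixStation widget to the viewport and plays the station-gone line.
; A second Refineries line follows after a short delay, and the widget is removed after a longer timed wait.
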(event EventBeginPlay
  (|CallParentFunction) ; This node is disabled and will not be called.\nDrag off pins to build functionality.
)

(event Collision|EventActorBeginOverlap
  (params (OtherActor :type Actor%20Object%20Reference))
  (|CallParentFunction OtherActor)
  (Utilities|Casting|CastToBP_Ship_Destroyer OtherActor)
  (Utilities|FlowControl|DoOnce false
    (:Completed
      (bind _returnvalue (UserInterface|CreateWidget "/Game/Assets/UI/OnboardingLevel/WP_HendrixStation.WP_HendrixStation_C"))
      (UserInterface|Viewport|AddtoViewport _returnvalue 0)
      (Audio|PlaySound2D "/Game/Assets/Audio/WAVs/VoiceLines/CorvetteVoiceLines/CorvetteStationGone_mixdown.CorvetteStationGone_mixdown" 1.0 1.0 0.0 0 0 false)
      (Utilities|FlowControl|Delay 3.0)
      (Audio|PlaySound2D "/Game/Assets/Audio/WAVs/VoiceLines/CmdrWhitlock/Refineries_mixdown.Refineries_mixdown" 1.0 1.0 0.0 0 0)
      (Utilities|FlowControl|Delay 1.2e+02)
      (Widget|RemovefromParent _returnvalue))))

(event EventTick
  (params (DeltaSeconds :type Float%20%28single-precision%29))
  (|CallParentFunction DeltaSeconds) ; This node is disabled and will not be called.\nDrag off pins to build functionality.
)

(fn ConstructionScript
  (|CallParentFunction))