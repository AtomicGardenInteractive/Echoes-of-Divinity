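; Trigger actor that plays the closing voice-line sequence of onboarding when the destroyer ship (BP_Ship_Destroyer) overlaps it.
; A DoOnce-gated overlap disables input on player controller 0, then plays the Whitlock blackbox, AI decryption and prepare-for-jump lines as 2D sounds spaced by fixed delays.
; It then adds the WP_OnboardingEnding widget to the viewport and calls EnableInput with no player controller argument.
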(event EventBeginPlay
  (|CallParentFunction) ; This node is disabled and will not be called.\nDrag off pins to build functionality.
)

(event Collision|EventActorBeginOverlap
  (params (OtherActor :type Actor%20Object%20Reference))
  (bind _returnvalue (Game|GetPlayerController 0))
  (|CallParentFunction OtherActor)
  (Utilities|Casting|CastToBP_Ship_Destroyer OtherActor)
  (Utilities|FlowControl|DoOnce false
    (:Completed
      (Input|DisableInput _returnvalue _returnvalue)
      (Audio|PlaySound2D "/Game/Assets/Audio/WAVs/VoiceLines/CmdrWhitlock/WhitlockBlackbox_mixdown.WhitlockBlackbox_mixdown" 1.0 1.0 0.0 0 0 false)
      (Utilities|FlowControl|Delay 5.0)
      (Audio|PlaySound2D "/Game/Assets/Audio/WAVs/VoiceLines/ShipAI/AIDecryption_mixdown.AIDecryption_mixdown" 1.0 1.0 0.0 0 0)
      (Utilities|FlowControl|Delay 19.0)
      (Audio|PlaySound2D "/Game/Assets/Audio/WAVs/VoiceLines/CmdrWhitlock/WhitlockPrepareForJump_mixdown.WhitlockPrepareForJump_mixdown" 1.0 1.0 0.0 0 0)
      (Utilities|FlowControl|Delay 5.0)
      (bind _returnvalue_2 (UserInterface|CreateWidget "/Game/Assets/UI/OnboardingLevel/WP_OnboardingEnding.WP_OnboardingEnding_C"))
      (UserInterface|Viewport|AddtoViewport _returnvalue_2 0)
      (Input|EnableInput (Game|GetPlayerController 0) 0))))

(event EventTick
  (params (DeltaSeconds :type Float%20%28single-precision%29))
  (|CallParentFunction DeltaSeconds) ; This node is disabled and will not be called.\nDrag off pins to build functionality.
)

(fn ConstructionScript
  (|CallParentFunction))