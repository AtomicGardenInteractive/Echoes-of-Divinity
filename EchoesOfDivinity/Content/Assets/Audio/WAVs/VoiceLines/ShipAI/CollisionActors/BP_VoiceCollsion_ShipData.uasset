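; A trigger actor that plays a scripted sequence of ship-data voice lines when the player's destroyer ship enters it.
; ActorBeginOverlap casts the other actor to BP_Ship_Destroyer, then a DoOnce gate lets the sequence run a single time.
; It plays the Whitlock ship data, Gilded Dawn and Whitlock ominous clips as 2D sounds, spaced by fixed delays.
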(event EventBeginPlay
  (|CallParentFunction) ; This node is disabled and will not be called.\nDrag off pins to build functionality.
)

(event Collision|EventActorBeginOverlap
  (params (OtherActor :type Actor%20Object%20Reference))
  (|CallParentFunction OtherActor)
  (Utilities|Casting|CastToBP_Ship_Destroyer OtherActor)
  (Utilities|FlowControl|DoOnce false
    (:Completed
      (Audio|PlaySound2D "/Game/Assets/Audio/WAVs/VoiceLines/CmdrWhitlock/WhitlockShipData_mixdown.WhitlockShipData_mixdown" 1.0 1.0 0.0 0 0 false)
      (Utilities|FlowControl|Delay 5.0)
      (Audio|PlaySound2D "/Game/Assets/Audio/WAVs/VoiceLines/ShipAI/GildedDawn_mixdown.GildedDawn_mixdown" 1.0 1.0 0.0 0 0)
      (Utilities|FlowControl|Delay 15.0)
      (Audio|PlaySound2D "/Game/Assets/Audio/WAVs/VoiceLines/CmdrWhitlock/WhitlockOminous_mixdown.WhitlockOminous_mixdown" 1.0 1.0 0.0 0 0))))

(event EventTick
  (params (DeltaSeconds :type Float%20%28single-precision%29))
  (|CallParentFunction DeltaSeconds) ; This node is disabled and will not be called.\nDrag off pins to build functionality.
)

(fn ConstructionScript
  (|CallParentFunction))