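; BP_VoiceCollsion_Intro is an actor that runs the timed intro sequence with voice lines and tutorial widgets as soon as play begins.
; BeginPlay disables player input and shows the camera controls widget while two 2D sounds, an AI line and the Whitlock intro, play between fixed delays.
; It then restores input and swaps to the ship selection widget, which is removed after a final delay.
; Despite the collision name, overlap only calls the parent.
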(event EventBeginPlay
  (bind _returnvalue (Game|GetPlayerController 0))
  (bind _returnvalue_2 (Game|GetPlayerController 0))
  (|CallParentFunction)
  (Input|DisableInput _returnvalue _returnvalue)
  (bind _returnvalue_3 (UserInterface|CreateWidget "/Game/Assets/UI/OnboardingLevel/WP_CameraControls.WP_CameraControls_C"))
  (UserInterface|Viewport|AddtoViewport _returnvalue_3 0)
  (Audio|PlaySound2D "/Game/Assets/Audio/WAVs/VoiceLines/ShipAI/AI15KM_mixdown.AI15KM_mixdown" 1.0 1.0 0.0 0 0 false)
  (Utilities|FlowControl|Delay 5.0)
  (Audio|PlaySound2D "/Game/Assets/Audio/WAVs/VoiceLines/CmdrWhitlock/WhitlockIntro_mixdown.WhitlockIntro_mixdown" 1.0 1.0 0.0 0 0)
  (Utilities|FlowControl|Delay 21.0)
  (Input|EnableInput _returnvalue_2 _returnvalue_2)
  (Utilities|FlowControl|Delay 1.5)
  (Widget|RemovefromParent _returnvalue_3)
  (bind _returnvalue_4 (UserInterface|CreateWidget "/Game/Assets/UI/OnboardingLevel/WP_ShipSelection.WP_ShipSelection_C"))
  (UserInterface|Viewport|AddtoViewport _returnvalue_4 0)
  (Utilities|FlowControl|Delay 2e+01)
  (Widget|RemovefromParent _returnvalue_4))

(event Collision|EventActorBeginOverlap
  (params (OtherActor :type Actor%20Object%20Reference))
  (|CallParentFunction OtherActor))

(event EventTick
  (params (DeltaSeconds :type Float%20%28single-precision%29))
  (|CallParentFunction DeltaSeconds) ; This node is disabled and will not be called.\nDrag off pins to build functionality.
)

(fn ConstructionScript
  (|CallParentFunction))