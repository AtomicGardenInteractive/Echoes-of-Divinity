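; A placeable voice-line trigger actor that reacts when a BP_Ship_Destroyer overlaps it, announcing detected vessels.
; A DoOnce gate makes the sequence fire a single time, adding a combat basics widget to the viewport and playing the AI detection line as 2D sound.
; After short delays it plays a Whitlock potential-contact line, then removes the widget.
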(event EventBeginPlay
  (|CallParentFunction) ; This node is disabled and will not be called.\nDrag off pins to build functionality.
)

(event Collision|EventActorBeginOverlap
  (params (OtherActor :type Actor%20Object%20Reference))
  (|CallParentFunction OtherActor)
  (Utilities|Casting|CastToBP_Ship_Destroyer OtherActor)
  (Utilities|FlowControl|DoOnce false
    (:Completed
      (bind _returnvalue (UserInterface|CreateWidget "/Game/Assets/UI/OnboardingLevel/WP_CombatBasics.WP_CombatBasics_C"))
      (UserInterface|Viewport|AddtoViewport _returnvalue 0)
      (Audio|PlaySound2D "/Game/Assets/Audio/WAVs/VoiceLines/ShipAI/AI_DetectedVessels_mixdown.AI_DetectedVessels_mixdown" 1.0 1.0 0.0 0 0 false)
      (Utilities|FlowControl|Delay 5.0)
      (Audio|PlaySound2D "/Game/Assets/Audio/WAVs/VoiceLines/CmdrWhitlock/WhitlockPotentialContactNew_mixdown.WhitlockPotentialContactNew_mixdown" 1.0 1.0 0.0 0 0)
      (Utilities|FlowControl|Delay 2e+01)
      (Widget|RemovefromParent _returnvalue))))

(event EventTick
  (params (DeltaSeconds :type Float%20%28single-precision%29))
  (|CallParentFunction DeltaSeconds) ; This node is disabled and will not be called.\nDrag off pins to build functionality.
)

(fn ConstructionScript
  (|CallParentFunction))