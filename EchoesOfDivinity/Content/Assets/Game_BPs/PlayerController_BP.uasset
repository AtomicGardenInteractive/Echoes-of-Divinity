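; Player controller for RTS-style ship control: click to select ships, then command them to move to a point under the cursor.
; Select traces under the cursor for a TestShip, adds it to SelectedShips and lights its indicator; K clears the selection.
; Contextual Command replaces any MoveMarker with one at the cursor trace hit, then sends each selected ship there via MoveOnServer and AIMoveTo, printing on failure.
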(event Custom|Add%20Ship
  (params (NewItem :type Pawn%20Object%20Reference%20%28by%20ref%29))
  ;[1 1 1] IS FINE
  (CallFunction|AddShiptoSelectedList NewItem))

(event Custom|Deselect%20All%20Ships
  (bind _arrayelement (Utilities|Array|ReverseforEachLoop (Variables|Default|GetSelected%20Ships))
    (:LoopBody
      (CallFunction|RemoveShipfromSelectedList _arrayelement))))

(event Custom|Remove%20Ship
  (params (NewItem :type Pawn%20Object%20Reference%20%28by%20ref%29))
  ;[1 1 1] IS FINE
  (CallFunction|RemoveShipfromSelectedList NewItem))

(event Custom|Move%20On%20Server
  (params (Pawn :type Pawn%20Object%20Reference) (Destination :type Vector))
  (bind _movementresult (AI|AIMoveTo Pawn Destination 0 5.0 true)
    (:OnFail
      (Development|PrintString (Utilities|String|EnumtoString _movementresult)))))

(event EventBeginPlay)

(event EventTick
  (params (DeltaSeconds :type Float%20%28single-precision%29)))

(event Input|ActionEvents|InputActionContextualCommand
  (params (Key :type Key%20Structure :default "None"))
  (:Pressed
    (bind _move_marker_transform (CallFunction|SpawnMoveMarker))
    (for _array_element (Variables|Default|GetSelected%20Ships)
      (CallFunction|MoveonServer _array_element _move_marker_transform))))

(event Input|ActionEvents|InputActionSelect
  (params (Key :type Key%20Structure :default "None"))
  (:Pressed
    (bind _astest_ship (Utilities|Casting|CastToTestShip (.HitActor (Collision|BreakHitResult (.HitResult (Class|PlayerController|GetHitResultUnderCursorforObjects (Utilities|Array|MakeArray "ObjectTypeQuery8") false))))))
    (CallFunction|AddShiptoSelectedList _astest_ship)
    (Default|SelectionIndicatoron _astest_ship)))

(event Input|KeyboardEvents|K
  (params (Key :type Key%20Structure :default "None"))
  (:Pressed
    (CallFunction|DeSelectAllShips)))

(fn ConstructionScript)

(fn AddShiptoSelectedList
  (params (New%20Ship%20Selection :type Pawn%20Object%20Reference%20%28by%20ref%29))
  (Utilities|Array|AddUnique (Variables|Default|GetSelected%20Ships) New%20Ship%20Selection))

(fn RemoveShipfromSelectedList
  (params (Item :type Pawn%20Object%20Reference%20%28by%20ref%29))
  (bind _astest_ship (Utilities|Casting|CastToTestShip Item))
  (Default|SelectionIndicatorOff _astest_ship)
  (Utilities|Array|RemoveItem (Variables|Default|GetSelected%20Ships) Item))

(fn SpawnMoveMarker
  (bind (_worldlocation _worlddirection) (Game|Player|ConvertMouseLocationToWorldSpace))
  (bind _outactors (Actor|GetAllActorsOfClass "/Game/Assets/3D/Blueprints/MoveMarker.MoveMarker_C"))
  (bind _arrayelement (Utilities|Array|ReverseforEachLoop _outactors)
    (:LoopBody
      (Actor|DestroyActor _arrayelement))
    (:Completed
      (bind (_outhit _returnvalue) (Collision|LineTraceByChannel _worldlocation (+ _worldlocation (* _worlddirection 5e+03)) "TraceTypeQuery1" false 0 "None"))
      (if _returnvalue
        (Game|SpawnActorfromClass "/Game/Assets/3D/Blueprints/MoveMarker.MoveMarker_C" (Math|Conversions|ToTransform(Vector) (.Location (Collision|BreakHitResult _outhit))) "AlwaysSpawn" (Game|GetPlayerController 0) 0)
        (return (.Location (Collision|BreakHitResult _outhit)))))))